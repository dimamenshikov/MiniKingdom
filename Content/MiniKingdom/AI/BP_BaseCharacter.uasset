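; Base character for MiniKingdom AI that handles life, death and a selectable info panel.
; BeginPlay binds the BPLife death event, creates a named info widget linked to BPLife, and clears the House reference if that house dies.
; Death hands mesh, scale and animation to a spawned BP_CharacterDeath, plays an optional sound and destroys the actor.
; Left-clicking toggles the widget in the interface's DopInfo panel.
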(event `Death`
  (params (Life :type "/Game/MiniKingdom/Blueprint/Components/BP_Life Object Reference"))
  (bind _mesh (`self.Mesh`))
  (bind _returnvalue (`|SpawnActorFromClass` "/Game/MiniKingdom/AI/BP_CharacterDeath.BP_CharacterDeath_C" (`self.GetTransform`) "Undefined" "MultiplyWithRoot" null null))
  (bind _skeletalmesh (`/Game/MiniKingdom/AI/BP_CharacterDeath.SkeletalMesh` _returnvalue))
  (`SceneComponent.SetWorldScale3D` _skeletalmesh (`SceneComponent.K2_GetComponentScale` _mesh))
  (`SkeletalMeshComponent.SetSkeletalMeshAsset` _skeletalmesh (`SkeletalMeshComponent.GetSkeletalMeshAsset` _mesh))
  (`/Game/MiniKingdom/AI/BP_CharacterDeath.Death` _returnvalue (`self.AnimDeath`))
  (bind _deathsound (`self.DeathSound`)
    (:`then`
      (`GameplayStatics.PlaySoundAtLocation` _deathsound (`self.K2_GetActorLocation`) (struct) 1.0 1.0 0.0 null null null null))
    (:`else`
      _))
  (`self.K2_DestroyActor`))

(event `self.ReceiveBeginPlay`
  (add `/Game/MiniKingdom/Blueprint/Components/BP_Life.OnDeath` (`self.BP_Life`) (`|CreateDelegate` :!event `Death`))
  (bind _returnvalue (`|CreateWidget` (`self.Class`)))
  (bind _output_get (set `self.WidgetObject` _returnvalue))
  (set `/Game/MiniKingdom/Blueprint/Components/BP_Life.Widget` _output_get (`self.BP_Life`))
  (`/Game/MiniKingdom/Widgets/WBP_AdvancedInfo.SetName` _output_get (`self.Name`))
  (bind _house (`self.House`)
    (:`then`
      (add `/Game/MiniKingdom/Blueprint/Components/BP_Life.OnDeath` (`/Game/MiniKingdom/Blueprint/Environment/BP_BaseBuilding.BP_Life` _house) (delegate `HouseDeath`)))
    (:`else`)))

(event `HouseDeath`
  (params (Life :type "/Game/MiniKingdom/Blueprint/Components/BP_Life Object Reference"))
  (set `self.House` null))

(event `/Game/MiniKingdom/Blueprint/Inteface/BPI_Click.LeftClick`
  (params (Interface :type "/Game/MiniKingdom/Widgets/WBP_Interface Object Reference") (Active :type Boolean))
  (bind _dopinfo (`/Game/MiniKingdom/Widgets/WBP_Interface.DopInfo` Interface))
  (bind _widgetobject (`self.WidgetObject`)
    (:`then`
      (if Active
        (`GameplayStatics.PlaySound2D` "/Engine/VREditor/Sounds/UI/Dockable_Window_Pick_Up.Dockable_Window_Pick_Up" 1.0 1.0 0.0 null null)
        (if (not (`PanelWidget.HasChild` _dopinfo (`self.WidgetObject`)))
          (`PanelWidget.ClearChildren` _dopinfo)
          (`PanelWidget.AddChild` _dopinfo _widgetobject))
        (else
          (`PanelWidget.RemoveChild` _dopinfo _widgetobject))))
    (:`else`)))

(fn `UserConstructionScript`)