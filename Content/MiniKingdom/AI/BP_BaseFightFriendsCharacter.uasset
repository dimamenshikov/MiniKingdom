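; Base AI character for friendly fighters in MiniKingdom, registering in the main castle's warrior list and sharing its task list.
; A weighted random roll picks relaxing at headquarters, patrolling, wandering research, or the castle task scoring highest by reward times coefficient.
; An active task takes priority, sending the warrior to attack or research.
; A looping timer heals through negative damage; warriors without headquarters retreat to the castle and are removed.
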(event `self.HouseDeath`
  (params (Life :type "/Game/MiniKingdom/Blueprint/Components/BP_Life Object Reference"))
  (`parent.HouseDeath` Life)
  (`self.Target`
    (:`then`)
    (:`else`
      (`/Game/MiniKingdom/Blueprint/Components/BP_KingdomPeople.GoToHouse` (`self.BP_FriendCharacter`) (`/Game/MiniKingdom/Blueprint/Components/BP_KingdomPeople.Main Castle` (`self.BP_FriendCharacter`))))))

(event `self.ReceiveBeginPlay`
  (`parent.ReceiveBeginPlay`)
  (bind _asbp_base_friend_building (cast `/Game/MiniKingdom/Blueprint/Environment/BP_BaseFriendBuilding` (`self.House`)))
  (set `self.Headquarter` _asbp_base_friend_building)
  (`KismetSystemLibrary.Delay` 0.2)
  (`self.Headquarter`
    (:`then`
      (add `/Game/MiniKingdom/Blueprint/Components/BP_KingdomPeople.OnInHouse` (`self.BP_FriendCharacter`) (delegate `InHouse`))
      (bind _maincastle (`/Game/MiniKingdom/Blueprint/DataAsset/PDA_Level.MainCastle` (`/Game/MiniKingdom/Blueprint/DataAsset/PDA_GameplayClasses.Level` (`/Game/MiniKingdom/Blueprint/Environment/BP_BaseBuilding.GameplayClasses` (`self.Headquarter`))))
        (:`then`
          (`KismetArrayLibrary.Array_Add` (`/Game/MiniKingdom/Blueprint/Environment/FriendBuilding/BP_MainCastle.Warriors` _maincastle) self)
          (set `self.Tasks` (`/Game/MiniKingdom/Blueprint/Environment/FriendBuilding/BP_MainCastle.Tasks` _maincastle))
          (`KismetSystemLibrary.K2_SetTimerDelegate` (delegate `Heal`) 0.5 true)
          (`KismetSystemLibrary.Delay` 1.0)
          (`self.Target`
            (:`then`)
            (:`else`
              (`self.SelectAction`))))
        (:`else`)))
    (:`else`)))

(event `Heal`
  (`GameplayStatics.ApplyDamage` self (* (`self.SpeedHeal`) -0.5)))

(event `InHouse`
  (`self.Headquarter`
    (:`then`
      (`KismetSystemLibrary.K2_SetTimerDelegate` (`|CreateDelegate` :!event `ExitHouse`) (`self.RelaxTime`)))
    (:`else`
      (bind _main_castle (`/Game/MiniKingdom/Blueprint/Components/BP_KingdomPeople.Main Castle` (`self.BP_FriendCharacter`))
        (:`then`
          (`KismetArrayLibrary.Array_RemoveItem` (`/Game/MiniKingdom/Blueprint/Environment/FriendBuilding/BP_MainCastle.Warriors` _main_castle) self)
          (`self.K2_DestroyActor`))
        (:`else`)))))

(event `self.EndPatrol`
  (`self.SelectAction`))

(event `Relax`
  (params (Time :type "Float (double-precision)"))
  (set `self.RelaxTime` Time)
  (`/Game/MiniKingdom/Blueprint/Components/BP_KingdomPeople.GoToHouse` (`self.BP_FriendCharacter`) (`self.Headquarter`)))

(event `self.Death`
  (params (Life :type "/Game/MiniKingdom/Blueprint/Components/BP_Life Object Reference"))
  (bind _returnvalue (`GameplayStatics.GetActorOfClass` "/Game/MiniKingdom/Blueprint/Environment/FriendBuilding/BP_MainCastle.BP_MainCastle_C"))
  (`/Engine/EditorBlueprintResources/StandardMacros.IsValid` _returnvalue
    (:`Is Valid`
      (`KismetArrayLibrary.Array_RemoveItem` (`/Game/MiniKingdom/Blueprint/Environment/FriendBuilding/BP_MainCastle.Warriors` _returnvalue) self))
    (:`Is Not Valid`
      _))
  (`parent.Death` null))

(event `self.SetTarget`
  (params (Target :type "Actor Object Reference"))
  (`KismetSystemLibrary.K2_ClearAndInvalidateTimerHandle` (`self.WaitResearchTimer`))
  (`parent.SetTarget` Target))

(event `SelectAction`
  (`self.ActiveTask`
    (:`then`
      (`self.Task` :!label _label))
    (:`else`
      (switch `int` (`self.Get Action`)
        (:`0`
          (`self.Relax` (`self.RelaxTime`)))
        (:`1`
          (`self.Patrol` (`self.PatrolCount`)))
        (:`2`
          (`self.Research` (`self.ResearchCount`)))
        (:`3`
          (goto _label))))))

(event `Task`
  (bind _activetask (`self.ActiveTask`))
  (`KismetArrayLibrary.Array_Add` (`/Game/MiniKingdom/Blueprint/Task/BP_BaseTask.ActiveCharacter` _activetask) self)
  (switch `/Game/MiniKingdom/Blueprint/Enum/E_Taks` (`/Game/MiniKingdom/Blueprint/Task/BP_BaseTask.Task` _activetask)
    (:`NewEnumerator0`
      (`self.SetTarget` (`self.GetOwner` (`self.ActiveTask`))))
    (:`NewEnumerator1`
      (`self.GoTo` (`self.K2_GetActorLocation` _activetask)))))

(event `self.GoToSuccess`
  (`self.Research` (`self.ResearchCount`)))

(event `Research`
  (params (ResearchCount :type Integer))
  (`self.SetWalk` true)
  (`self.Target` :!label _label_2
    (:`then`)
    (:`else`
      (`|AIMoveTo` self (+ (`self.K2_GetActorLocation`) (`KismetMathLibrary.GreaterGreater_VectorRotator` (`KismetMathLibrary.MakeVector` (`KismetMathLibrary.RandomFloatInRange` (`self.InnerRadiusResearch`) (`self.OutRadiusResearch`))) (`KismetMathLibrary.MakeRotator` 0.0 0.0 (`KismetMathLibrary.RandomFloatInRange` -180.0 180.0)))) null 10.0
        (:`OnSuccess`
          (bind _returnvalue (`KismetSystemLibrary.K2_SetTimerDelegate` (`|CreateDelegate` :!event `EndResearch`) (`KismetMathLibrary.RandomFloatInRange` 2.0 5.0)))
          (set `self.WaitResearchTimer` _returnvalue))
        (:`OnFail`
          (`KismetSystemLibrary.Delay` 1.0)
          (if (not (!= (`MovementComponent.Velocity` (`self.CharacterMovement`)) (0.0 0.0 0.0) :`ErrorTolerance` 0.01))
            (goto _label_2)))))))

(event `EndResearch`
  (bind _returnvalue (- (stale `Research` ResearchCount) 1))
  (if (> _returnvalue 0)
    (`self.Research` _returnvalue)
    (else
      (`self.SelectAction`))))

(event `ExitHouse`
  (`/Game/MiniKingdom/Blueprint/Components/BP_Life.Health` (`self.BP_Life`))
  (`/Game/MiniKingdom/Blueprint/Components/BP_KingdomPeople.ExitOfHouse` (`self.BP_FriendCharacter`))
  (`self.SelectAction`))

(event `self.NoMoreTarget`
  (bind _headquarter (`self.Headquarter`)
    (:`then`
      (remove `self.OnTakeAnyDamage` _headquarter (`|CreateDelegate` :!event `HouseAttack`))
      (`self.SelectAction`))
    (:`else`
      (`/Game/MiniKingdom/Blueprint/Components/BP_KingdomPeople.GoToHouse` (`self.BP_FriendCharacter`) (`/Game/MiniKingdom/Blueprint/Components/BP_KingdomPeople.Main Castle` (`self.BP_FriendCharacter`))))))

(fn `Get Action`
  (returns (`Array Index` :type Integer))
  (locals (Random :type Integer :default 0) (NewLocalVar :type Integer))
  (bind _array (`|MakeArray` (`self.RelaxChance`) (`self.PatrolChance`) (`self.ResearchChance`) (`self.GetChanceTask`)))
  (for _array_element _array
    (set `local.NewLocalVar` (+ _array_element (`local.NewLocalVar`))))
  (set `local.Random` (`KismetMathLibrary.RandomInteger` (`local.NewLocalVar`)))
  (set `local.NewLocalVar` 0)
  (for (_array_element_2 _array_index) _array
    (bind _returnvalue (+ _array_element_2 (`local.NewLocalVar`)))
    (if (> _returnvalue (`local.Random`))
      (return _array_index)
      (else
        (set `local.NewLocalVar` _returnvalue)))))

(fn `GetChanceTask`
  (returns (ResultChanceTask :type Integer))
  (locals (index :type Integer :default 0))
  (bind _tasks (`self.Tasks`))
  (bind _output (`|GetArrayItem` _tasks (`local.index`)))
  (bind _returnvalue (* (`/Game/MiniKingdom/Blueprint/Task/BP_BaseTask.Reward` _output) (`BlueprintMapLibrary.Map_Find` (`self.CoefficientTask`) (`/Game/MiniKingdom/Blueprint/Task/BP_BaseTask.Task` _output))))
  (if (`KismetArrayLibrary.Array_IsNotEmpty` (`self.Tasks`))
    (for (_array_element _array_index) _tasks
      (`/Engine/EditorBlueprintResources/StandardMacros.IsValid` _array_element
        (:`Is Valid`
          (`/Engine/EditorBlueprintResources/StandardMacros.IsValid` _output
            (:`Is Valid`
              (if (> (* (`BlueprintMapLibrary.Map_Find` (`self.CoefficientTask`) (`/Game/MiniKingdom/Blueprint/Task/BP_BaseTask.Task` _array_element)) (`/Game/MiniKingdom/Blueprint/Task/BP_BaseTask.Reward` _array_element)) _returnvalue)
                (set `local.index` _array_index)))))))
    (`/Engine/EditorBlueprintResources/StandardMacros.IsValid` _output
      (:`Is Valid`
        (set `self.ActiveTask` _output)
        (return (/ _returnvalue 10)))
      (:`Is Not Valid`
        (return -1)))
    (else
      (return -1))))

(fn `UserConstructionScript`
  (`parent.UserConstructionScript`))