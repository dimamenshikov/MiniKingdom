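; Base AI fighter for MiniKingdom that patrols around its House and fights characters or buildings.
; Visible-zone overlaps, damage taken and House damage set targets; target death selects the nearest overlapping actor or resumes patrol.
; Pursuit uses AIMoveTo, re-issued through a gate for characters, with range measured to a GetPoint location on buildings.
; In range, a looping timer plays the attack montage, whose notify spawns a HitClass actor carrying damage and target.
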(event `self.ReceiveBeginPlay`
  (`parent.ReceiveBeginPlay`))

(event `self.Visible.OnComponentBeginOverlap`
  (params (OverlappedComponent :type "PrimitiveComponent Object Reference") (OtherActor :type "Actor Object Reference") (OtherComp :type "PrimitiveComponent Object Reference") (OtherBodyIndex :type Integer) (bFromSweep :type Boolean) (SweepResult :type "HitResult Structure (by ref)"))
  (`self.Target`
    (:`then`
      (`self.Building`
        (:`then`
          _)
        (:`else`)))
    (:`else`
      _))
  (`self.SetTarget` OtherActor))

(event `TargetDeath`
  (params (Life :type "/Game/MiniKingdom/Blueprint/Components/BP_Life Object Reference"))
  (set `self.DamagedActor` null)
  (set `self.Building` null)
  (set `self.Target` null)
  (`self.StopAnimMontage` (`AnimInstance.GetCurrentActiveMontage` (`SkeletalMeshComponent.GetAnimInstance` (`self.Mesh`))))
  (`KismetSystemLibrary.K2_ClearAndInvalidateTimerHandle` (`self.Hits`))
  (set `self.CanHit` true)
  (`self.CheckTargets`))

(event `PursueCharacter`
  (set `self.Fight` false)
  (`|ExecutionSequence`
    (:`then_0`
      (goto _label :!via `Open`))
    (:`then_1`
      (`/Engine/EditorBlueprintResources/StandardMacros.Gate` true :!label _label
        (:`Exit`
          (`self.Target`
            (:`then`
              (bind _target (`self.CheckDistanceAttack`)
                (:`CanAttack`
                  (`|ExecutionSequence` :!label _label_2
                    (:`then_0`
                      (goto _label :!via `Close`))
                    (:`then_1`
                      (`self.Attack`))))
                (:`NoCanAttack`
                  (`|AIMoveTo` self _target null (`self.AttackDistance`)
                    (:`then`
                      (`KismetSystemLibrary.DelayUntilNextTick`)
                      (goto _label))
                    (:`OnSuccess`
                      (goto _label_2))
                    (:`OnFail`
                      (`KismetSystemLibrary.Delay` 1.0)
                      (if (not (!= (`MovementComponent.Velocity` (`self.CharacterMovement`)) (0.0 0.0 0.0) :`ErrorTolerance` 0.01))
                        (goto _label)))))))
            (:`else`)))))))

(event `EndPatrol`
  (`self.Patrol` (`self.PatrolCount`)))

(event `NoMoreTarget`
  (bind _house (`self.House`)
    (:`then`
      (remove `self.OnTakeAnyDamage` _house (`|CreateDelegate` :!event `HouseAttack`))
      (`self.Patrol` (`self.PatrolCount`)))
    (:`else`)))

(event `CheckTargets`
  (bind _newtarget (`self.Get New Target`))
  (`/Engine/EditorBlueprintResources/StandardMacros.IsValid` _newtarget
    (:`Is Valid`
      (`self.SetTarget` _newtarget))
    (:`Is Not Valid`
      (set `self.Target` null)
      (`self.NoMoreTarget`))))

(event `PursueBuilding`
  (bind _target (`self.CheckDistanceAttack`)
    (:`CanAttack`
      _)
    (:`NoCanAttack`
      (`|AIMoveTo` self _target null (`KismetMathLibrary.FMax` (- (`self.AttackDistance`) 100.0) 50.0)
        (:`OnSuccess`
          _))))
  (`self.Attack`))

(event `RotateToTarget`
  (bind _target (`self.Target`)
    (:`then`
      (bind (_returnvalue_roll _returnvalue_pitch _returnvalue_yaw) (`KismetMathLibrary.BreakRotator` (`KismetMathLibrary.FindLookAtRotation` (`self.K2_GetActorLocation`) (`self.K2_GetActorLocation` _target))))
      (`self.K2_SetActorRotation` (`KismetMathLibrary.MakeRotator` 0.0 0.0 _returnvalue_yaw)))
    (:`else`)))

(event `self.ReceiveAnyDamage`
  (params (Damage :type "Float (single-precision)") (DamageType :type "DamageType Object Reference") (InstigatedBy :type "Controller Object Reference") (DamageCauser :type "Actor Object Reference"))
  (`/Engine/EditorBlueprintResources/StandardMacros.IsValid` DamageCauser
    (:`Is Valid`
      (`self.DamagedActor`
        (:`then`)
        (:`else`
          (bind _output_get (set `self.DamagedActor` DamageCauser))
          (if (!= DamageCauser (`self.Target`))
            (`self.SetTarget` _output_get)))))))

(event `GoTo`
  (params (Target :type "Vector Structure"))
  (`self.SetWalk` true)
  (`|AIMoveTo` self Target null 10.0
    (:`OnSuccess`
      _)
    (:`OnFail`
      _))
  (`self.GoToSuccess`))

(event `GoToSuccess`)

(event `SetWalk`
  (params (Patrol :type Boolean))
  (bind _output_get (set `self.CanPatrol` Patrol))
  (set `self.Fight` false)
  (set `CharacterMovementComponent.MaxWalkSpeed` (`KismetMathLibrary.SelectFloat` (`self.SpeedPatrol`) (`self.SpeedFight`) _output_get) (`self.CharacterMovement`))
  (`KismetSystemLibrary.K2_ClearAndInvalidateTimerHandle` (`self.WaitTimer`)))

(event `HouseAttack` :!signature `self.OnTakeAnyDamage`
  (params (DamagedActor :type "Actor Object Reference") (Damage :type "Float (single-precision)") (DamageType :type "DamageType Object Reference") (InstigatedBy :type "Controller Object Reference") (DamageCauser :type "Actor Object Reference"))
  (if (> Damage 0.0)
    (`self.Target`
      (:`then`)
      (:`else`
        (`self.SetTarget` DamageCauser)))))

(event `Patrol`
  (params (Count :type Integer))
  (bind (_returnvalue_x _returnvalue_y) (`KismetMathLibrary.BreakVector` (`SceneComponent.K2_GetComponentScale` (`/Game/MiniKingdom/Blueprint/Environment/BP_BaseBuilding.BlockZone` (`self.House`)))))
  (`self.SetWalk` true)
  (bind _house (`self.House`)
    (:`then`
      (add `self.OnTakeAnyDamage` _house (`|CreateDelegate` :!event `HouseAttack`))
      (if (`self.CanPatrol`) :!label _label_3
        (bind _house_2 (`self.House`)
          (:`then`
            (`|AIMoveTo` self (+ (`KismetMathLibrary.GreaterGreater_VectorRotator` (`KismetMathLibrary.MakeVector` (`KismetMathLibrary.RandomFloatInRange` (* (`KismetMathLibrary.FMax` _returnvalue_x _returnvalue_y) 60.0) (`self.RadiusPatrol`))) (`KismetMathLibrary.MakeRotator` 0.0 0.0 (`KismetMathLibrary.RandomFloatInRange` 180.0 -180.0))) (`self.K2_GetActorLocation` _house_2)) null 10.0
              (:`OnSuccess`
                (bind _returnvalue (`KismetSystemLibrary.K2_SetTimerDelegate` (`|CreateDelegate` :!event `NewPatrol`) (`KismetMathLibrary.RandomFloatInRange` 2.0 4.0)))
                (set `self.WaitTimer` _returnvalue))
              (:`OnFail`
                (`KismetSystemLibrary.Delay` 1.0)
                (if (not (!= (`MovementComponent.Velocity` (`self.CharacterMovement`)) (0.0 0.0 0.0) :`ErrorTolerance` 0.01))
                  (goto _label_3)))))
          (:`else`))))
    (:`else`)))

(event `NewPatrol`
  (bind _returnvalue (- (stale `Patrol` Count) 1))
  (if (> _returnvalue 0)
    (`self.Patrol` _returnvalue)
    (else
      (bind _house (`self.House`)
        (:`then`
          (remove `self.OnTakeAnyDamage` _house (`|CreateDelegate` :!event `HouseAttack`)))
        (:`else`
          _))
      (`self.EndPatrol`))))

(event `Attack`
  (if (`self.CanHit`)
    (set `self.CanHit` false)
    (`self.RotateToTarget`)
    (set `self.Fight` true)
    (`self.Hit`)
    (bind _returnvalue (`KismetSystemLibrary.K2_SetTimerDelegate` (`|CreateDelegate` :!event `Hit`) 1.0 true))
    (set `self.Hits` _returnvalue)))

(event `SetTarget`
  (params (Target :type "Actor Object Reference"))
  (bind _returnvalue (`self.GetComponentByClass` (`self.Target`) "/Game/MiniKingdom/Blueprint/Components/BP_Life.BP_Life_C"))
  (`/Engine/EditorBlueprintResources/StandardMacros.IsValid` Target
    (:`Is Valid`
      (`self.Target`
        (:`then`
          (remove `/Game/MiniKingdom/Blueprint/Components/BP_Life.OnDeath` _returnvalue (`|CreateDelegate` :!event `TargetDeath`)))
        (:`else`
          _))
      (bind _output_get (set `self.Target` Target))
      (add `/Game/MiniKingdom/Blueprint/Components/BP_Life.OnDeath` _returnvalue (`|CreateDelegate` :!event `TargetDeath`))
      (`MovementComponent.StopMovementImmediately` (`self.CharacterMovement`))
      (`self.SetWalk` false)
      (bind _asbp_base_building (cast `/Game/MiniKingdom/Blueprint/Environment/BP_BaseBuilding` _output_get)
        (:`then`
          (set `self.Building` _asbp_base_building)
          (`self.PursueBuilding`))
        (:`CastFailed`
          (set `self.Building` null)
          (`self.PursueCharacter`))))))

(event `Hit`
  (bind _hits (`self.Hits`))
  (`self.Target`
    (:`then`
      (`self.Building`
        (:`then`
          (`|PlayMontage` (`self.Mesh`) (`self.AnimAttack`) :!label _label_4
            (:`OnNotifyBegin`
              (`self.RotateToTarget`)
              (bind _target (`self.Target`)
                (:`then`
                  (`|SpawnActorFromClass` (`self.HitClass`) (`self.GetTransform`) "AlwaysSpawn" "MultiplyWithRoot" self (`self.Damage`) _target null))
                (:`else`)))))
        (:`else`
          (`self.CheckDistanceAttack`
            (:`CanAttack`
              (goto _label_4))
            (:`NoCanAttack`
              (`KismetSystemLibrary.K2_ClearAndInvalidateTimerHandle` _hits)
              (set `self.CanHit` true)
              (`self.PursueCharacter`))))))
    (:`else`
      (`KismetSystemLibrary.K2_ClearAndInvalidateTimerHandle` _hits)
      (set `self.CanHit` true))))

(fn `Get New Target`
  (returns (NewTarget :type "Actor Object Reference"))
  (locals (VisibilityActors :type "Array of Actor Object Reference"))
  (return (`.ReturnValue` (`GameplayStatics.FindNearestActor` (`self.K2_GetActorLocation`) (`PrimitiveComponent.GetOverlappingActors` (`self.Visible`) "/Script/Engine.Actor")))))

(fn `UserConstructionScript`
  (`parent.UserConstructionScript`))