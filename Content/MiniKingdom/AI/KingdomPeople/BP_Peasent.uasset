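; Peasant character that repairs damaged buildings of the main castle in MiniKingdom.
; Castle building events report attacks and new construction; an idle peasant takes the attacked building, otherwise picks a random damaged one.
; It walks there, retrying failed moves if stationary, then a per-frame timer heals through negative ApplyDamage with hammer sounds.
; On full health or building death it seeks another target, returning to the castle when none remain.
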(event `self.ReceiveBeginPlay`
  (bind _maincastle (`/Game/MiniKingdom/Blueprint/DataAsset/PDA_Level.MainCastle` (`self.Level`)))
  (`parent.ReceiveBeginPlay`)
  (add `/Game/MiniKingdom/Blueprint/Environment/FriendBuilding/BP_MainCastle.OnNewBuilding` _maincastle (delegate `NewBuilding`))
  (for _array_element (`/Game/MiniKingdom/Blueprint/Environment/FriendBuilding/BP_MainCastle.Building` _maincastle)
    (add `/Game/MiniKingdom/Blueprint/Environment/BP_BaseFriendBuilding.OnAttack` _array_element (`|CreateDelegate` :!event `BuildingAttacked`)))
  (`self.CheckBuildings` null))

(event `NewBuilding`
  (params (NewBuilding :type "/Game/MiniKingdom/Blueprint/Environment/BP_BaseFriendBuilding Object Reference"))
  (add `/Game/MiniKingdom/Blueprint/Environment/BP_BaseFriendBuilding.OnAttack` NewBuilding (`|CreateDelegate` :!event `BuildingAttacked`)))

(event `BuildingAttacked`
  (params (Building :type "/Game/MiniKingdom/Blueprint/Environment/BP_BaseFriendBuilding Object Reference"))
  (`self.FixBuilding`
    (:`then`)
    (:`else`
      (set `self.FixBuilding` Building)
      (`self.Move`))))

(event `Move`
  (`/Game/MiniKingdom/Blueprint/Components/BP_KingdomPeople.ExitOfHouse` (`self.BP_FriendCharacter`))
  (set `self.CanFix` false)
  (set `self.Fight` false)
  (add `/Game/MiniKingdom/Blueprint/Components/BP_Life.OnDeath` (`/Game/MiniKingdom/Blueprint/Environment/BP_BaseBuilding.BP_Life` (`self.FixBuilding`)) (`|CreateDelegate` :!event `CheckBuildings`))
  (bind _returnvalue (`KismetSystemLibrary.K2_SetTimerDelegate` (`|CreateDelegate` :!event `Fix`) (`GameplayStatics.GetWorldDeltaSeconds`) true))
  (set `self.FixTimer` _returnvalue)
  (bind _fixbuilding (`self.FixBuilding` :!label _label)
    (:`then`
      (bind _returnvalue_2 (`/Game/MiniKingdom/Blueprint/Environment/BP_BaseBuilding.Get Point` _fixbuilding (`self.K2_GetActorLocation`)))
      (`|AIMoveTo` self _returnvalue_2 null 10.0
        (:`OnSuccess`
          (`self.K2_SetActorRotation` (`KismetMathLibrary.FindLookAtRotation` (`self.K2_GetActorLocation`) (`self.K2_GetActorLocation` _fixbuilding)))
          (set `self.Fight` true)
          (set `self.CanFix` true))
        (:`OnFail`
          (`KismetSystemLibrary.Delay` 0.5)
          (if (not (!= (`MovementComponent.Velocity` (`self.CharacterMovement`)) (0.0 0.0 0.0) :`ErrorTolerance` 0.01))
            (goto _label)))))
    (:`else`)))

(event `Fix`
  (bind _fixbuilding (`self.FixBuilding`)
    (:`then`
      (if (`/Game/MiniKingdom/Blueprint/Components/BP_Life.IsMaxHealth` (`/Game/MiniKingdom/Blueprint/Environment/BP_BaseBuilding.BP_Life` _fixbuilding))
        (`KismetSystemLibrary.K2_ClearAndInvalidateTimerHandle` (`self.FixTimer`))
        (remove `/Game/MiniKingdom/Blueprint/Components/BP_Life.OnDeath` (`/Game/MiniKingdom/Blueprint/Environment/BP_BaseBuilding.BP_Life` (`self.FixBuilding`)) (`|CreateDelegate` :!event `CheckBuildings`))
        (`self.CheckBuildings` null)
        (elif (`self.CanFix`)
          (`GameplayStatics.ApplyDamage` (`self.FixBuilding`) (* (`GameplayStatics.GetWorldDeltaSeconds`) (`self.Fixed`) -1.0))
          (`KismetSystemLibrary.Delay` 1.0)
          (`self.FixBuilding`
            (:`then`
              (`GameplayStatics.PlaySoundAtLocation` "/Game/MiniKingdom/Assets/Sound/A_Hammer.A_Hammer" (`self.K2_GetActorLocation`) (struct) 1.0 1.0 0.0 null null null null))
            (:`else`)))))
    (:`else`)))

(event `CheckBuildings`
  (params (Life :type "/Game/MiniKingdom/Blueprint/Components/BP_Life Object Reference"))
  (bind _buildingtemp (`self.BuildingTemp`))
  (`KismetSystemLibrary.K2_ClearAndInvalidateTimerHandle` (`self.FixTimer`))
  (set `self.FixBuilding` null)
  (`KismetArrayLibrary.Array_Clear` (`self.BuildingTemp`))
  (for _array_element (`/Game/MiniKingdom/Blueprint/Environment/FriendBuilding/BP_MainCastle.Building` (`/Game/MiniKingdom/Blueprint/DataAsset/PDA_Level.MainCastle` (`self.Level`)))
    (bind _bp_life (`/Game/MiniKingdom/Blueprint/Environment/BP_BaseBuilding.BP_Life` _array_element))
    (if (and (`/Game/MiniKingdom/Blueprint/Components/BP_Life.IsLive` _bp_life) (not (`/Game/MiniKingdom/Blueprint/Components/BP_Life.IsMaxHealth` _bp_life)))
      (`KismetArrayLibrary.Array_Add` (`self.BuildingTemp`) _array_element)))
  (if (`KismetArrayLibrary.Array_IsNotEmpty` _buildingtemp)
    (set `self.FixBuilding` (`KismetArrayLibrary.Array_Random` _buildingtemp))
    (`self.Move`)
    (else
      (`/Game/MiniKingdom/Blueprint/Components/BP_KingdomPeople.GoToHouse` (`self.BP_FriendCharacter`) (`/Game/MiniKingdom/Blueprint/DataAsset/PDA_Level.MainCastle` (`self.Level`))))))

(fn `UserConstructionScript`
  (`parent.UserConstructionScript`))