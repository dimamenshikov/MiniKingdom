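; BP_Guard is a MiniKingdom guard AI that defends the main castle and its buildings.
; On BeginPlay it binds to damage events on the castle and its existing buildings, and to the castle's new-building event so later buildings are covered too.
; Any positive damage makes the damage causer its target unless it already has a valid one.
; With a valid castle and no target after a short delay, it starts patrolling.
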(event `self.ReceiveBeginPlay`
  (`parent.ReceiveBeginPlay`)
  (bind _maincastle (`/Game/MiniKingdom/Blueprint/DataAsset/PDA_Level.MainCastle` (`/Game/MiniKingdom/Blueprint/DataAsset/PDA_GameplayClasses.Level` (`/Game/MiniKingdom/Blueprint/Environment/BP_BaseBuilding.GameplayClasses` (`self.House`))))
    (:`then`
      (add `/Game/MiniKingdom/Blueprint/Environment/FriendBuilding/BP_MainCastle.OnNewBuilding` _maincastle (delegate `CastleAttack`))
      (add `Actor.OnTakeAnyDamage` _maincastle (delegate `BuildingAttack`))
      (for _array_element (`/Game/MiniKingdom/Blueprint/Environment/FriendBuilding/BP_MainCastle.Building` _maincastle)
        (add `Actor.OnTakeAnyDamage` _array_element (delegate `BuildingAttack`)))
      (`KismetSystemLibrary.Delay` 1.0)
      (`self.Target`
        (:`then`)
        (:`else`
          (`self.Patrol` 5))))
    (:`else`)))

(event `CastleAttack`
  (params (NewBuilding :type "/Game/MiniKingdom/Blueprint/Environment/BP_BaseFriendBuilding Object Reference"))
  (add `Actor.OnTakeAnyDamage` NewBuilding (delegate `BuildingAttack`)))

(event `BuildingAttack`
  (params (DamagedActor :type "Actor Object Reference") (Damage :type "Float (single-precision)") (DamageType :type "DamageType Object Reference") (InstigatedBy :type "Controller Object Reference") (DamageCauser :type "Actor Object Reference"))
  (if (> Damage 0.0)
    (`self.Target`
      (:`then`)
      (:`else`
        (`self.SetTarget` DamageCauser)))))

(fn `UserConstructionScript`
  (`parent.UserConstructionScript`))