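; BP_Collector is a kingdom worker that gathers gold from buildings and brings it to the main castle.
; A five-second timer queues non-castle buildings holding over 250 gold, then the collector visits random queued entries via AI MoveTo, retrying failed moves when stationary.
; When none remain it returns to the castle, where the in-house event deposits gold and restarts the timer.
; A targeted building's death event drops it and picks another.
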(event `self.ReceiveBeginPlay`
  (`parent.ReceiveBeginPlay`)
  (add `/Game/MiniKingdom/Blueprint/Components/BP_KingdomPeople.OnInHouse` (`self.BP_FriendCharacter`) (delegate `InHouse`))
  (`self.SetTimerForCheckGold`))

(event `InHouse`
  (`/Game/MiniKingdom/Blueprint/Components/BP_KingdomPeople.GiveGold` (`self.BP_FriendCharacter`))
  (`self.SetTimerForCheckGold`))

(event `SetTimerForCheckGold`
  (`KismetSystemLibrary.K2_SetTimerDelegate` (delegate `CheckGold`) 5.0))

(event `CheckGold`
  (bind _maincastle (`/Game/MiniKingdom/Blueprint/DataAsset/PDA_Level.MainCastle` (`/Game/MiniKingdom/Blueprint/DataAsset/PDA_GameplayClasses.Level` (`/Game/MiniKingdom/Blueprint/Environment/BP_BaseBuilding.GameplayClasses` (`self.House`)))))
  (for _array_element (`/Game/MiniKingdom/Blueprint/Environment/FriendBuilding/BP_MainCastle.Building` _maincastle)
    (if (and (!= _maincastle _array_element) (> (`/Game/MiniKingdom/Blueprint/Environment/BP_BaseFriendBuilding.Gold` _array_element) 250))
      (`KismetArrayLibrary.Array_Add` (`self.BuildingTemp`) _array_element)))
  (`self.MoveTakeGold`))

(event `MoveTakeGold`
  (bind _targetbuilding (`self.TargetBuilding`))
  (bind _targetbuilding_2 (`self.TargetBuilding`))
  (bind _output_get (set `self.TargetBuilding` (`KismetArrayLibrary.Array_Random` (`self.BuildingTemp`))))
  (`/Engine/EditorBlueprintResources/StandardMacros.IsValid` _output_get
    (:`Is Valid`
      (`/Game/MiniKingdom/Blueprint/Components/BP_KingdomPeople.ExitOfHouse` (`self.BP_FriendCharacter`))
      (add `/Game/MiniKingdom/Blueprint/Components/BP_Life.OnDeath` (`/Game/MiniKingdom/Blueprint/Environment/BP_BaseBuilding.BP_Life` _targetbuilding_2) (delegate `BuildingDeath`))
      (`|AIMoveTo` self (`SceneComponent.K2_GetComponentLocation` (`/Game/MiniKingdom/Blueprint/Environment/BP_BaseBuilding.Entrance` _targetbuilding_2)) null 10.0 :!label _label
        (:`OnSuccess`
          (`/Game/MiniKingdom/Blueprint/Components/BP_KingdomPeople.TakeGold` (`self.BP_FriendCharacter`) _targetbuilding)
          (`KismetArrayLibrary.Array_RemoveItem` (`self.BuildingTemp`) _targetbuilding)
          (`self.MoveTakeGold`))
        (:`OnFail`
          (`KismetSystemLibrary.Delay` 0.5)
          (if (not (!= (`MovementComponent.Velocity` (`self.CharacterMovement`)) (0.0 0.0 0.0) :`ErrorTolerance` 0.01))
            (goto _label)))))
    (:`Is Not Valid`
      (`/Game/MiniKingdom/Blueprint/Components/BP_KingdomPeople.GoToHouse` (`self.BP_FriendCharacter`) (`/Game/MiniKingdom/Blueprint/DataAsset/PDA_Level.MainCastle` (`/Game/MiniKingdom/Blueprint/DataAsset/PDA_GameplayClasses.Level` (`/Game/MiniKingdom/Blueprint/Environment/BP_BaseBuilding.GameplayClasses` (`self.House`))))))))

(event `BuildingDeath`
  (params (Life :type "/Game/MiniKingdom/Blueprint/Components/BP_Life Object Reference"))
  (`KismetArrayLibrary.Array_RemoveItem` (`self.BuildingTemp`) (`self.TargetBuilding`))
  (`self.MoveTakeGold`))

(fn `UserConstructionScript`
  (`parent.UserConstructionScript`))