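; BP_BaseEnemyCharacter is the base enemy AI character that patrols from its House and later attacks the main castle.
; With a valid House it caches the castle and patrols; otherwise it walks to a point on the found castle.
; When movement, patrol or targets end, it targets the castle if Day exceeds DaysAttack or House is gone; house death also triggers this.
; Right-click spawns a task actor and shows its widget, destroying unattached tasks on deselection.
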(event `self.ReceiveBeginPlay`
  (`parent.ReceiveBeginPlay`)
  (bind _house (`self.House`)
    (:`then`
      (bind _maincastle (`/Game/MiniKingdom/Blueprint/DataAsset/PDA_Level.MainCastle` (`/Game/MiniKingdom/Blueprint/DataAsset/PDA_GameplayClasses.Level` (`/Game/MiniKingdom/Blueprint/Environment/BP_BaseBuilding.GameplayClasses` _house)))
        (:`then`
          (set `self.Main Castle` _maincastle)
          (`self.Patrol` (`self.PatrolCount`)))
        (:`else`)))
    (:`else`
      (bind _returnvalue (`GameplayStatics.GetActorOfClass` "/Game/MiniKingdom/Blueprint/Environment/FriendBuilding/BP_MainCastle.BP_MainCastle_C"))
      (`/Engine/EditorBlueprintResources/StandardMacros.IsValid` _returnvalue
        (:`Is Valid`
          (bind _returnvalue_2 (`/Game/MiniKingdom/Blueprint/Environment/BP_BaseBuilding.Get Point` _returnvalue (`self.K2_GetActorLocation`)))
          (`self.GoTo` _returnvalue_2))))))

(event `/Game/MiniKingdom/Blueprint/Inteface/BPI_Click.RightClick`
  (params (Interface :type "/Game/MiniKingdom/Widgets/WBP_Interface Object Reference") (Active :type Boolean))
  (bind (_returnvalue_x _returnvalue_y) (`KismetMathLibrary.BreakVector` (`self.K2_GetActorLocation`)))
  (bind _dopinfo (`/Game/MiniKingdom/Widgets/WBP_Interface.DopInfo` Interface))
  (if Active
    (`self.Task`
      (:`then`
        _)
      (:`else`
        (bind _returnvalue (`|SpawnActorFromClass` "/Game/MiniKingdom/Blueprint/Task/BP_BaseTask.BP_BaseTask_C" (`KismetMathLibrary.MakeTransform` (`KismetMathLibrary.MakeVector` _returnvalue_x _returnvalue_y 90.0)) "AlwaysSpawn" "MultiplyWithRoot" self "NewEnumerator0" null))
        (bind _output_get (set `self.Task` _returnvalue))
        (`SceneComponent.K2_SetRelativeLocation` (`/Game/MiniKingdom/Blueprint/Task/BP_BaseTask.StaticMesh` _output_get) (0.0 0.0 1000.0) false false)))
    (`PanelWidget.ClearChildren` _dopinfo)
    (`PanelWidget.AddChild` _dopinfo (`/Game/MiniKingdom/Blueprint/Task/BP_BaseTask.Widget` _output_get))
    (else
      (bind _task (`self.Task`)
        (:`then`
          (if (`/Game/MiniKingdom/Blueprint/Task/BP_BaseTask.Attach` _task)
            (`PanelWidget.ClearChildren` _dopinfo)
            (else
              (`self.K2_DestroyActor` _task))))
        (:`else`)))))

(event `self.GoToSuccess`
  (`self.Main Castle`
    (:`then`
      (if (> (`/Game/MiniKingdom/Blueprint/Environment/FriendBuilding/BP_MainCastle.Day` (`self.Main Castle`)) (`self.DaysAttack`)) :!label _label
        (bind _main_castle (`self.Main Castle` :!label _label_2)
          (:`then`
            (`self.SetTarget` _main_castle))
          (:`else`))
        (else
          (`self.House`
            (:`then`
              (`self.Patrol` (`self.PatrolCount`)))
            (:`else`
              (goto _label_2))))))
    (:`else`)))

(event `self.HouseDeath`
  (params (Life :type "/Game/MiniKingdom/Blueprint/Components/BP_Life Object Reference"))
  (`parent.HouseDeath` Life)
  (goto _label_2))

(event `self.NoMoreTarget`
  (`self.Main Castle`
    (:`then`
      (goto _label))
    (:`else`)))

(event `self.EndPatrol`
  (`self.Main Castle`
    (:`then`
      (goto _label))
    (:`else`)))

(fn `UserConstructionScript`
  (`parent.UserConstructionScript`))