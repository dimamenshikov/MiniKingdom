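; Game mode for MiniKingdom that starts level music, handles mission messages, pausing and the end-of-game screen.
; It watches the main castle's destruction, then after a short delay shows defeat text and ends the game as a loss.
; Mission texts appear as a chain of info widgets, each close opening the next until the OnInfoNoMore dispatcher fires.
; Pause toggles game state and notifies the HUD.
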(event `self.ReceiveBeginPlay`
  (set `/Game/MiniKingdom/Blueprint/DataAsset/PDA_GameplayClasses.GM` self (`self.GameplayClasses`))
  (`GameplayStatics.PlaySound2D` "/Game/MiniKingdom/Assets/Sound/A_LevelMusic.A_LevelMusic" 1.0 1.0 0.0 null null)
  (bind _returnvalue (`|CreateWidget` "/Game/MiniKingdom/Widgets/WBP_LevelInfo.WBP_LevelInfo_C"))
  (set `self.Widget` _returnvalue)
  (bind _returnvalue_2 (`GameplayStatics.GetActorOfClass` "/Game/MiniKingdom/Blueprint/Environment/FriendBuilding/BP_MainCastle.BP_MainCastle_C"))
  (add `self.OnDestroyed` _returnvalue_2 (delegate `CastleDeath`)))

(event `CastleDeath` :!signature `self.OnDestroyed`
  (params (DestroyedActor :type "Actor Object Reference"))
  (`KismetSystemLibrary.Delay` 2.0)
  (add `self.OnInfoNoMore` (delegate `Defeat`))
  (`self.ShowMissionInfo` (`|MakeArray` (`self.DefeatInfo`))))

(event `Defeat`
  (`self.EndGame` false))

(event `ShowMissionInfo`
  (params (Texts :type "Array of Text") (Index :type Integer))
  (bind _returnvalue (`|CreateWidget` "/Game/MiniKingdom/Widgets/WBP_LevelInfo.WBP_LevelInfo_C"))
  (`UserWidget.AddToViewport` _returnvalue 0)
  (set `TextBlock.Text` (`|GetArrayItem` Texts Index) (`/Game/MiniKingdom/Widgets/WBP_LevelInfo.TextMission` _returnvalue))
  (add `/Game/MiniKingdom/Widgets/WBP_LevelInfo.OnCloseInfo` _returnvalue (delegate `NextInfo`)))

(event `NextInfo`
  (bind _returnvalue (+ (stale `ShowMissionInfo` Index) 1))
  (if (>= (`KismetArrayLibrary.Array_LastIndex` (stale `ShowMissionInfo` Texts)) _returnvalue)
    (`self.ShowMissionInfo` (stale `ShowMissionInfo` Texts) _returnvalue)
    (else
      (`self.OnInfoNoMore`))))

(event `EndGame`
  (params (Win :type Boolean))
  (`GameplayStatics.SetGamePaused` true)
  (bind _returnvalue (`|CreateWidget` "/Game/MiniKingdom/Widgets/WBP_EndGame.WBP_EndGame_C" null Win))
  (`UserWidget.AddToViewport` _returnvalue 0))

(fn `SetPause`
  (`GameplayStatics.SetGamePaused` (not (`GameplayStatics.IsGamePaused`)))
  (`/Game/MiniKingdom/Core/BP_MiniKingdom_HUD.SetPause` (`/Game/MiniKingdom/Blueprint/DataAsset/PDA_GameplayClasses.HUD` (`self.GameplayClasses`)) (`GameplayStatics.IsGamePaused`)))

(fn `UserConstructionScript`)