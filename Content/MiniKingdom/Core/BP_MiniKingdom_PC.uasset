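; MiniKingdom player controller that creates the main UI and handles top-down management camera control, selection and orders.
; Edge scrolling, wheel zoom, middle-drag pan and right-drag rotation feed PlayerMove, which limits height and pitch on the pawn.
; Left click selects the attached or hovered actor through click messages, deactivating the previous one.
; Right click deselects, messages the hovered actor or spawns a BP_BaseTask; a short timer suppresses this after drags.
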(event `self.ReceiveBeginPlay`
  (`WidgetBlueprintLibrary.SetInputMode_GameAndUIEx` self null "LockAlways")
  (set `/Game/MiniKingdom/Blueprint/DataAsset/PDA_GameplayClasses.PC` self (`self.GameplayClasses`))
  (`EnhancedInputSubsystemInterface.AddMappingContext` (subsystem `EnhancedInputLocalPlayerSubsystem`) "/Game/MiniKingdom/Input/IMC_Management.IMC_Management" 0 (struct))
  (bind _returnvalue (`|CreateWidget` "/Game/MiniKingdom/Widgets/WBP_Interface.WBP_Interface_C"))
  (bind _output_get (set `self.Interface` _returnvalue))
  (`UserWidget.AddToViewport` _output_get 0))

(event `self.ReceiveTick`
  (params (DeltaSeconds :type "Float (single-precision)"))
  (if (and (not (`|GetInputActionValue`)) (not (`|GetInputActionValue`)))
    (`/Game/MiniKingdom/Blueprint/DataAsset/PDA_GameplayClasses.P` (`self.GameplayClasses`)
      (:`then`
        (`self.Look`))
      (:`else`))))

(event `EnhancedInput|/Game/MiniKingdom/Input/Action/IA_ClickLeft`
  (params (ActionValue :type Boolean) (ElapsedSeconds :type "Float (double-precision)") (TriggeredSeconds :type "Float (double-precision)") (InputAction :type "InputAction Object Reference" :default "/Game/MiniKingdom/Input/Action/IA_ClickLeft.IA_ClickLeft"))
  (bind _hit_result_hit_actor (`self.Hit Result Hit Actor`))
  (:`Started`
    (bind _attachactor (`self.AttachActor`)
      (:`then`
        (message `/Game/MiniKingdom/Blueprint/Inteface/BPI_Click.LeftClick` _attachactor (`self.Interface`) true)
        (if (!= _attachactor (`self.ActorActive`))
          (`self.DeatctiveActor` (`self.ActorActive`))
          (set `self.ActorActive` null)))
      (:`else`
        (bind _output_get (set `self.Hit Result Hit Actor` (`.HitActor` (`GameplayStatics.BreakHitResult` (`self.GetHitResultUnderCursorByChannel` "TraceTypeQuery3")))))
        (`/Engine/EditorBlueprintResources/StandardMacros.IsValid` _output_get
          (:`Is Valid`
            (`self.ActorActive`
              (:`then`
                (if (!= (`self.ActorActive`) _output_get)
                  (`self.DeatctiveActor` (`self.ActorActive`))))
              (:`else`
                _))
            (set `self.ActorActive` _hit_result_hit_actor)
            (message `/Game/MiniKingdom/Blueprint/Inteface/BPI_Click.LeftClick` _hit_result_hit_actor (`self.Interface`) true))
          (:`Is Not Valid`
            (`self.DeatctiveActor` (`self.ActorActive`))
            (set `self.ActorActive` null)))))))

(event `EnhancedInput|/Game/MiniKingdom/Input/Action/IA_ClickRight`
  (params (ActionValue :type Boolean) (ElapsedSeconds :type "Float (double-precision)") (TriggeredSeconds :type "Float (double-precision)") (InputAction :type "InputAction Object Reference" :default "/Game/MiniKingdom/Input/Action/IA_ClickRight.IA_ClickRight"))
  (bind _hitresult (`self.GetHitResultUnderCursorByChannel` "TraceTypeQuery3"))
  (bind _dopinfo (`/Game/MiniKingdom/Widgets/WBP_Interface.DopInfo` (`self.Interface`)))
  (:`Completed`
    (`KismetSystemLibrary.K2_ClearAndInvalidateTimerHandle` (`self.Timer`))
    (if (`self.CanOrder`)
      (bind _actoractive (`self.ActorActive`)
        (:`then`
          (`self.DeatctiveActor` _actoractive)
          (set `self.ActorActive` null))
        (:`else`
          (`/Engine/EditorBlueprintResources/StandardMacros.IsValid` (`.HitActor` (`GameplayStatics.BreakHitResult` _hitresult))
            (:`Is Valid`
              (message `/Game/MiniKingdom/Blueprint/Inteface/BPI_Click.RightClick` (`.HitActor` (`GameplayStatics.BreakHitResult` _hitresult)) (`self.Interface`) true))
            (:`Is Not Valid`
              (bind _returnvalue (`|SpawnActorFromClass` "/Game/MiniKingdom/Blueprint/Task/BP_BaseTask.BP_BaseTask_C" (`KismetMathLibrary.MakeTransform` (`KismetMathLibrary.MakeVector` (.x (`.Location` (`GameplayStatics.BreakHitResult` (`self.GetHitResultUnderCursorByChannel` "TraceTypeQuery4")))) (.y (`.Location` (`GameplayStatics.BreakHitResult` (`self.GetHitResultUnderCursorByChannel` "TraceTypeQuery4")))))) "AlwaysSpawn" "MultiplyWithRoot" null "NewEnumerator1" null))
              (`PanelWidget.ClearChildren` _dopinfo)
              (`PanelWidget.AddChild` _dopinfo (`/Game/MiniKingdom/Blueprint/Task/BP_BaseTask.Widget` _returnvalue))))))
      (else
        (set `self.CanOrder` true)))))

(event `EnhancedInput|/Game/MiniKingdom/Input/Action/IA_Wheel`
  (params (ActionValue :type "Float (double-precision)") (ElapsedSeconds :type "Float (double-precision)") (TriggeredSeconds :type "Float (double-precision)") (InputAction :type "InputAction Object Reference" :default "/Game/MiniKingdom/Input/Action/IA_Wheel.IA_Wheel"))
  (bind _p (`/Game/MiniKingdom/Blueprint/DataAsset/PDA_GameplayClasses.P` (`self.GameplayClasses`)))
  (:`Triggered`
    (`self.PlayerMove` (+ (* (* ActionValue 500.0) (`self.GetActorForwardVector` _p)) (`self.K2_GetActorLocation` _p)))))

(event `EnhancedInput|/Game/MiniKingdom/Input/Action/IA_Pause`
  (params (ActionValue :type Boolean) (ElapsedSeconds :type "Float (double-precision)") (TriggeredSeconds :type "Float (double-precision)") (InputAction :type "InputAction Object Reference" :default "/Game/MiniKingdom/Input/Action/IA_Pause.IA_Pause"))
  (:`Started`
    (`/Game/MiniKingdom/Core/BP_MiniKingdom_GM.SetPause` (`/Game/MiniKingdom/Blueprint/DataAsset/PDA_GameplayClasses.GM` (`self.GameplayClasses`)))))

(event `ProhibitOrder`
  (set `self.CanOrder` false))

(event `EnhancedInput|/Game/MiniKingdom/Input/Action/IA_Look`
  (params (ActionValue :type "Vector2D Structure") (ElapsedSeconds :type "Float (double-precision)") (TriggeredSeconds :type "Float (double-precision)") (InputAction :type "InputAction Object Reference" :default "/Game/MiniKingdom/Input/Action/IA_Look.IA_Look"))
  (bind (_returnvalue_x _returnvalue_y) (`KismetMathLibrary.BreakVector2D` (* ActionValue 5.0)))
  (bind (_returnvalue_roll _returnvalue_pitch _returnvalue_yaw) (`KismetMathLibrary.BreakRotator` (`self.K2_GetActorRotation` (`/Game/MiniKingdom/Blueprint/DataAsset/PDA_GameplayClasses.P` (`self.GameplayClasses`)))))
  (:`Triggered`
    (if (`|GetInputActionValue`)
      (if (`self.CanOrder`)
        (bind _returnvalue (`KismetSystemLibrary.K2_SetTimerDelegate` (delegate `ProhibitOrder`) 0.05))
        (set `self.Timer` _returnvalue))
      (`self.PlayerMove` (0.0 0.0 6000.0) (`KismetMathLibrary.MakeRotator` 0.0 (+ _returnvalue_y _returnvalue_pitch) (+ _returnvalue_yaw _returnvalue_x 0.0))))))

(event `EnhancedInput|/Game/MiniKingdom/Input/Action/IA_WheelAxis`
  (params (ActionValue :type "Vector2D Structure") (ElapsedSeconds :type "Float (double-precision)") (TriggeredSeconds :type "Float (double-precision)") (InputAction :type "InputAction Object Reference" :default "/Game/MiniKingdom/Input/Action/IA_WheelAxis.IA_WheelAxis"))
  (bind (_returnvalue_x _returnvalue_y) (`KismetMathLibrary.BreakVector` (`KismetMathLibrary.Conv_Vector2DToVector` ActionValue)))
  (bind _p (`/Game/MiniKingdom/Blueprint/DataAsset/PDA_GameplayClasses.P` (`self.GameplayClasses`)))
  (bind (_returnvalue_roll _returnvalue_pitch _returnvalue_yaw) (`KismetMathLibrary.BreakRotator` (`self.K2_GetActorRotation` _p)))
  (:`Triggered`
    (if (`|GetInputActionValue`)
      (`self.PlayerMove` (+ (`KismetMathLibrary.GreaterGreater_VectorRotator` (* (`KismetMathLibrary.MakeVector` _returnvalue_y _returnvalue_x) -50.0) (`KismetMathLibrary.MakeRotator` 0.0 0.0 _returnvalue_yaw)) (`self.K2_GetActorLocation` _p))))))

(fn `DeatctiveActor`
  (params (Actor :type "Actor Object Reference"))
  (bind _interface (`self.Interface`))
  (`/Engine/EditorBlueprintResources/StandardMacros.IsValid` Actor
    (:`Is Valid`
      (message `/Game/MiniKingdom/Blueprint/Inteface/BPI_Click.LeftClick` Actor _interface false)
      (`/Engine/EditorBlueprintResources/StandardMacros.IsValid` Actor
        (:`Is Valid`
          (message `/Game/MiniKingdom/Blueprint/Inteface/BPI_Click.RightClick` Actor _interface false))))))

(fn `Look`
  (locals (Move :type "Vector Structure") (NewLocalVar :type "Vector Structure" :default (0.0 0.0 0.0)))
  (bind (_locationx _locationy) (`self.GetMousePosition`))
  (bind (_returnvalue_x _returnvalue_y) (`KismetMathLibrary.BreakVector2D` (`WidgetLayoutLibrary.GetViewportSize`)))
  (bind _p (`/Game/MiniKingdom/Blueprint/DataAsset/PDA_GameplayClasses.P` (`self.GameplayClasses`)))
  (bind (_returnvalue_roll _returnvalue_pitch _returnvalue_yaw) (`KismetMathLibrary.BreakRotator` (`self.K2_GetActorRotation` _p)))
  (bind _output_get (set `local.Move` (`KismetMathLibrary.MakeVector` (`KismetMathLibrary.SelectFloat` (`KismetMathLibrary.SelectFloat` 10.0 -10.0 (<= _locationy 2.0)) 0.0 (or (< _locationy 2.0) (`KismetMathLibrary.NearlyEqual_FloatFloat` _locationy _returnvalue_y 2.0))) (`KismetMathLibrary.SelectFloat` (`KismetMathLibrary.SelectFloat` -10.0 10.0 (<= _locationx 2.0)) 0.0 (or (< _locationx 2.0) (`KismetMathLibrary.NearlyEqual_FloatFloat` _locationx _returnvalue_x 2.0))))))
  (if (!= _output_get (0.0 0.0 0.0) :`ErrorTolerance` 0.001)
    (`self.PlayerMove` (+ (`KismetMathLibrary.GreaterGreater_VectorRotator` (* (`local.Move`) (`self.SpeedCameraMove`)) (`KismetMathLibrary.MakeRotator` 0.0 0.0 _returnvalue_yaw)) (`self.K2_GetActorLocation` _p)))))

(fn `PlayerMove`
  (params (NewLocation :type "Vector Structure" :default (0.0 0.0 6000.0)) (NewRotation :type "Rotator Structure" :default (struct :`Roll` 100.0)))
  (bind _p (`/Game/MiniKingdom/Blueprint/DataAsset/PDA_GameplayClasses.P` (`self.GameplayClasses`)))
  (if (and (`KismetMathLibrary.InRange_FloatFloat` (.z NewLocation) 1000.0 4000.0) (!= NewLocation (0.0 0.0 6000.0)))
    (`self.K2_SetActorLocation` _p NewLocation true false))
  (if (!= NewRotation (struct :`Roll` 100.0))
    (`self.K2_SetActorRotation` _p (`KismetMathLibrary.MakeRotator` 0.0 (`KismetMathLibrary.FClamp` (.pitch NewRotation) -85.0 -35.0) (.yaw NewRotation)) false)))

(fn `SetActiveActor`
  (params (Actor :type "Actor Object Reference"))
  (`/Engine/EditorBlueprintResources/StandardMacros.IsValid` Actor
    (:`Is Valid`
      (if (!= (`self.ActorActive`) Actor)
        (`self.DeatctiveActor` (`self.ActorActive`)))
      (set `self.ActorActive` Actor))))

(fn `UserConstructionScript`)