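; BP_BeginBuilding is the placement preview for buying a building in MiniKingdom.
; On spawn it checks affordability with the MainCastle, registers as the controller's active actor and takes its meshes from the building class data.
; Each tick it follows the cursor, turning red when its neighborhood zone overlaps actors or the trace misses.
; An active left click rechecks, spawns the building, charges gold and registers it; right click cancels.
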(event `self.ReceiveBeginPlay`
  (bind _buildingmesh (`self.BuildingMesh`))
  (bind _classbuilding (`self.ClassBuilding`))
  (bind _neighborhoodzone (`self.NeighborhoodZone`))
  (bind _canbuy (`/Game/MiniKingdom/Blueprint/Environment/FriendBuilding/BP_MainCastle.CanBuyBuilding` (`/Game/MiniKingdom/Blueprint/DataAsset/PDA_Level.MainCastle` (`/Game/MiniKingdom/Blueprint/DataAsset/PDA_GameplayClasses.Level` (`self.GameplayClasses`))) (`/Game/MiniKingdom/Blueprint/DataAsset/PDA_Building.Class` (`self.ClassBuilding`))))
  (if _canbuy
    (set `/Game/MiniKingdom/Core/BP_MiniKingdom_PC.ActorActive` self (`/Game/MiniKingdom/Blueprint/DataAsset/PDA_GameplayClasses.PC` (`self.GameplayClasses`)))
    (`StaticMeshComponent.SetStaticMesh` _neighborhoodzone (`/Game/MiniKingdom/Blueprint/DataAsset/PDA_Building.NeighborhoodZone` (`self.ClassBuilding`)))
    (`SceneComponent.SetWorldScale3D` _neighborhoodzone (`/Game/MiniKingdom/Blueprint/DataAsset/PDA_Building.NeighborhoodZoneScale` (`self.ClassBuilding`)))
    (`StaticMeshComponent.SetStaticMesh` _buildingmesh (`/Game/MiniKingdom/Blueprint/DataAsset/PDA_Building.BuildingMesh` _classbuilding))
    (`SceneComponent.K2_SetRelativeTransform` _buildingmesh (`/Game/MiniKingdom/Blueprint/DataAsset/PDA_Building.BuildingMeshTransform` _classbuilding) false false)
    (set `self.Material` (`MeshComponent.GetMaterials` (`self.BuildingMesh`)))
    (else
      (`self.K2_DestroyActor`))))

(event `self.ReceiveTick`
  (params (DeltaSeconds :type "Float (single-precision)"))
  (bind _buildingmesh (`self.BuildingMesh`))
  (bind _hitresult (`PlayerController.GetHitResultUnderCursorByChannel` (`/Game/MiniKingdom/Blueprint/DataAsset/PDA_GameplayClasses.PC` (`self.GameplayClasses`)) "TraceTypeQuery4" true))
  (`self.K2_SetActorLocationAndRotation` (`.Location` (`GameplayStatics.BreakHitResult` _hitresult)) (struct :`Yaw` 180.0) true)
  (set `self.CanBuild` (and (`KismetArrayLibrary.Array_IsEmpty` (`PrimitiveComponent.GetOverlappingActors` (`self.NeighborhoodZone`) "/Script/Engine.Actor")) (`GameplayStatics.BreakHitResult` _hitresult)))
  (for (_ _array_index) (`MeshComponent.GetMaterials` _buildingmesh)
    (`PrimitiveComponent.SetMaterial` _buildingmesh _array_index (select `bool` (`self.CanBuild`) :`false` "/Game/MiniKingdom/Assets/GlobalMaterial/MI_Red.MI_Red" :`true` (`|GetArrayItem` (`self.Material`) _array_index)))))

(event `/Game/MiniKingdom/Blueprint/Inteface/BPI_Click.LeftClick`
  (params (Interface :type "/Game/MiniKingdom/Widgets/WBP_Interface Object Reference") (Active :type Boolean))
  (bind _maincastle (`/Game/MiniKingdom/Blueprint/DataAsset/PDA_Level.MainCastle` (`/Game/MiniKingdom/Blueprint/DataAsset/PDA_GameplayClasses.Level` (`self.GameplayClasses`))))
  (if Active
    (bind _maincastle_2 (`/Game/MiniKingdom/Blueprint/DataAsset/PDA_Level.MainCastle` (`/Game/MiniKingdom/Blueprint/DataAsset/PDA_GameplayClasses.Level` (`self.GameplayClasses`)))
      (:`then`
        (bind (_canbuy _cost) (`/Game/MiniKingdom/Blueprint/Environment/FriendBuilding/BP_MainCastle.CanBuyBuilding` _maincastle_2 (`/Game/MiniKingdom/Blueprint/DataAsset/PDA_Building.Class` (`self.ClassBuilding`))))
        (if (and _canbuy (`self.CanBuild`))
          (bind _returnvalue (`|SpawnActorFromClass` (`/Game/MiniKingdom/Blueprint/DataAsset/PDA_Building.Class` (`self.ClassBuilding`)) (`self.GetTransform`) "AlwaysSpawn" "MultiplyWithRoot" null null))
          (`/Game/MiniKingdom/Blueprint/Environment/BP_BaseFriendBuilding.AddGold` _maincastle _cost false)
          (`/Game/MiniKingdom/Blueprint/Environment/FriendBuilding/BP_MainCastle.AddBuilding` _maincastle _returnvalue)
          (`GameplayStatics.PlaySound2D` "/Game/MiniKingdom/Assets/Sound/A_Building.A_Building" 1.0 1.0 0.0 null null)
          (`self.K2_DestroyActor`)
          (else
            (`GameplayStatics.PlaySound2D` "/Game/MiniKingdom/Assets/Sound/A_Error.A_Error" 1.0 1.0 0.0 null null))))
      (:`else`))
    (else
      (`self.K2_DestroyActor`))))

(event `/Game/MiniKingdom/Blueprint/Inteface/BPI_Click.RightClick`
  (params (Interface :type "/Game/MiniKingdom/Widgets/WBP_Interface Object Reference") (Active :type Boolean))
  (`self.K2_DestroyActor`))

(fn `UserConstructionScript`)