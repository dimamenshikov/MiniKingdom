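; Player's main castle, the kingdom's hub that tracks gold, days, buildings and warrior tasks, updating the interface and broadcasting new days and buildings.
; On BeginPlay it registers with the level, starts a looping day timer and spawns guards, collectors and peasants up to caps, replacing them on death.
; Building purchases have per-class limits and exponentially rising costs.
; When the castle dies, it triggers death for all its kingdom people.
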(event `self.ReceiveBeginPlay`
  (bind _gameplayclasses (`self.GameplayClasses`))
  (bind _level (`/Game/MiniKingdom/Blueprint/DataAsset/PDA_GameplayClasses.Level` _gameplayclasses))
  (set `/Game/MiniKingdom/Blueprint/DataAsset/PDA_Level.MainCastle` self _level)
  (`parent.ReceiveBeginPlay`)
  (`KismetArrayLibrary.Array_Add` (`self.Building`) self)
  (bind _output_get (set `self.Gold` (`/Game/MiniKingdom/Blueprint/DataAsset/PDA_Level.StartGold` _level)))
  (`KismetSystemLibrary.DelayUntilNextTick`)
  (`/Game/MiniKingdom/Widgets/WBP_Interface.SetGold` (`/Game/MiniKingdom/Core/BP_MiniKingdom_PC.Interface` (`/Game/MiniKingdom/Blueprint/DataAsset/PDA_GameplayClasses.PC` _gameplayclasses)) _output_get)
  (`self.SpawnGuard`)
  (`self.SpawnCollector`)
  (`self.SpawnPeasant`)
  (bind _returnvalue (`KismetSystemLibrary.K2_SetTimerDelegate` (`|CreateDelegate` :!event `IncreaseGold`) 5.0 true))
  (set `self.DaysTimer` _returnvalue)
  (`self.IncreaseGold`)
  (`/Game/MiniKingdom/Blueprint/Components/BP_Life.Health` (`self.BP_Life`)))

(event `IncreaseGold`
  (bind _result (`/Engine/EditorBlueprintResources/StandardMacros.IncrementInt` (`self.Day`))
    (:`  `
      (`/Game/MiniKingdom/Widgets/WBP_Interface.SetDay` (`/Game/MiniKingdom/Core/BP_MiniKingdom_PC.Interface` (`/Game/MiniKingdom/Blueprint/DataAsset/PDA_GameplayClasses.PC` (`self.GameplayClasses`))) _result)
      (`self.OnNewDay` _result))))

(event `SpawnGuard`
  (if (< (`self.QuantityGuard`) (`self.QuantityGuardBorder`))
    (bind _returnvalue (`|SpawnActorFromClass` "/Game/MiniKingdom/AI/KingdomPeople/BP_Guard.BP_Guard_C" (`SceneComponent.K2_GetComponentToWorld` (`self.Entrance`)) "AlwaysSpawn" "MultiplyWithRoot" null self null))
    (add `/Game/MiniKingdom/Blueprint/Components/BP_Life.OnDeath` (`/Game/MiniKingdom/AI/BP_BaseCharacter.BP_Life` _returnvalue) (delegate `GuardDeath`))
    (`/Engine/EditorBlueprintResources/StandardMacros.IncrementInt` (`self.QuantityGuard`)
      (:`  `
        (`KismetSystemLibrary.Delay` 3.0)
        (`self.SpawnGuard`)))))

(event `GuardDeath`
  (params (Life :type "/Game/MiniKingdom/Blueprint/Components/BP_Life Object Reference"))
  (`/Engine/EditorBlueprintResources/StandardMacros.DecrementInt` (`self.QuantityGuard`)
    (:`  `
      (`KismetSystemLibrary.Delay` 3.0)
      (`self.SpawnGuard`))))

(event `SpawnCollector`
  (if (< (`self.QuantityCollector`) (`self.QuantityCollectorBorder`))
    (bind _returnvalue (`|SpawnActorFromClass` "/Game/MiniKingdom/AI/KingdomPeople/BP_Collector.BP_Collector_C" (`SceneComponent.K2_GetComponentToWorld` (`self.Entrance`)) "AlwaysSpawn" "MultiplyWithRoot" null self null))
    (bind _bp_friendcharacter (`/Game/MiniKingdom/AI/KingdomPeople/BP_Collector.BP_FriendCharacter` _returnvalue))
    (`/Game/MiniKingdom/Blueprint/Components/BP_KingdomPeople.HiddenCharacter` _bp_friendcharacter true)
    (set `/Game/MiniKingdom/Blueprint/Components/BP_KingdomPeople.InBuilding` self _bp_friendcharacter)
    (add `/Game/MiniKingdom/Blueprint/Components/BP_Life.OnDeath` (`/Game/MiniKingdom/AI/BP_BaseCharacter.BP_Life` _returnvalue) (delegate `DeathCollector`))
    (`/Engine/EditorBlueprintResources/StandardMacros.IncrementInt` (`self.QuantityCollector`)
      (:`  `
        (`KismetSystemLibrary.Delay` 3.0)
        (`self.SpawnCollector`)))))

(event `DeathCollector`
  (params (Life :type "/Game/MiniKingdom/Blueprint/Components/BP_Life Object Reference"))
  (`/Engine/EditorBlueprintResources/StandardMacros.DecrementInt` (`self.QuantityCollector`)
    (:`  `
      (`KismetSystemLibrary.Delay` 3.0)
      (`self.SpawnCollector`))))

(event `SpawnPeasant`
  (if (< (`self.QuantityPeasant`) (`self.QuantityPeasantBorder`))
    (bind _returnvalue (`|SpawnActorFromClass` "/Game/MiniKingdom/AI/KingdomPeople/BP_Peasent.BP_Peasent_C" (`SceneComponent.K2_GetComponentToWorld` (`self.Entrance`)) "AlwaysSpawn" "MultiplyWithRoot" null self null))
    (bind _bp_friendcharacter (`/Game/MiniKingdom/AI/KingdomPeople/BP_Peasent.BP_FriendCharacter` _returnvalue))
    (`/Game/MiniKingdom/Blueprint/Components/BP_KingdomPeople.HiddenCharacter` _bp_friendcharacter true)
    (set `/Game/MiniKingdom/Blueprint/Components/BP_KingdomPeople.InBuilding` self _bp_friendcharacter)
    (add `/Game/MiniKingdom/Blueprint/Components/BP_Life.OnDeath` (`/Game/MiniKingdom/AI/BP_BaseCharacter.BP_Life` _returnvalue) (delegate `DeathPeasant`))
    (`/Engine/EditorBlueprintResources/StandardMacros.IncrementInt` (`self.QuantityPeasant`)
      (:`  `
        (`KismetSystemLibrary.Delay` 3.0)
        (`self.SpawnPeasant`)))))

(event `DeathPeasant`
  (params (Life :type "/Game/MiniKingdom/Blueprint/Components/BP_Life Object Reference"))
  (`/Engine/EditorBlueprintResources/StandardMacros.DecrementInt` (`self.QuantityPeasant`)
    (:`  `
      (`KismetSystemLibrary.Delay` 3.0)
      (`self.SpawnPeasant`))))

(event `self.Death`
  (for _array_element (`self.KingdomPeople`)
    (bind _bp_life (`/Game/MiniKingdom/AI/BP_BaseCharacter.BP_Life` (`/Game/MiniKingdom/Blueprint/Components/BP_KingdomPeople.BaseCharacter` _array_element)))
    (`/Game/MiniKingdom/Blueprint/Components/BP_Life.OnDeath` _bp_life _bp_life))
  (`parent.Death`))

(event `/Game/MiniKingdom/Blueprint/Inteface/BPI_Click.LeftClick`
  (params (Interface :type "/Game/MiniKingdom/Widgets/WBP_Interface Object Reference") (Active :type Boolean))
  (set `WidgetSwitcher.ActiveWidgetIndex` 0 (`/Game/MiniKingdom/Widgets/WBP_Interface.WidgetSwitcher` Interface)))

(fn `AddBuilding`
  (params (Building :type "/Game/MiniKingdom/Blueprint/Environment/BP_BaseFriendBuilding Object Reference"))
  (`KismetArrayLibrary.Array_Add` (`self.Building`) Building)
  (`self.OnNewBuilding` Building))

(fn `AddGold`
  (params (Delta :type Integer) (Add :type Boolean))
  (`parent.AddGold` Delta Add)
  (`/Game/MiniKingdom/Widgets/WBP_Interface.SetGold` (`/Game/MiniKingdom/Core/BP_MiniKingdom_PC.Interface` (`/Game/MiniKingdom/Blueprint/DataAsset/PDA_GameplayClasses.PC` (`self.GameplayClasses`))) (`self.Gold`)))

(fn `CanBuyBuilding`
  (params (Building :type "/Game/MiniKingdom/Blueprint/Environment/BP_BaseFriendBuilding Class Reference"))
  (returns (CanBuy :type Boolean) (Cost :type Integer))
  (locals (Quantity :type Integer))
  (bind _returnvalue (* (defaults `Object` Building) (`KismetMathLibrary.MultiplyMultiply_FloatFloat` 1.5 (`KismetMathLibrary.Conv_IntToDouble` (`local.Quantity`)))))
  (for _array_element (`self.Building`)
    (if (== Building (`GameplayStatics.GetObjectClass` _array_element))
      (`/Engine/EditorBlueprintResources/StandardMacros.IncrementInt` (`local.Quantity`))))
  (if (< (`local.Quantity`) (`BlueprintMapLibrary.Map_Find` (`self.QuantityBorderBuilding`) Building))
    (return (<= _returnvalue (`self.Gold`)) _returnvalue)
    (else
      (return false 0))))

(fn `CanBuySimpleObject`
  (params (Cost :type Integer))
  (returns (CanBuy :type Boolean))
  (return (<= Cost (`self.Gold`))))

(fn `NewTasks`
  (params (Task :type "/Game/MiniKingdom/Blueprint/Task/BP_BaseTask Object Reference"))
  (`KismetArrayLibrary.Array_Add` (`self.Tasks`) Task)
  (for _array_element (`self.Warriors`)
    (`KismetArrayLibrary.Array_Add` (`/Game/MiniKingdom/AI/BP_BaseFightFriendsCharacter.Tasks` _array_element) Task)))

(fn `UserConstructionScript`)