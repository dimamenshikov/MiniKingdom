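; BP_DefenceTower is a buildable friendly tower that fires arrows at actors inside its Visible detection component.
; Once built, it targets the nearest overlapping actor, or a new entrant when idle, and retargets when the target leaves or becomes invalid.
; A looping recharge timer spawns BP_HitArrow toward the target, passing damage and target.
; Shortly after BeginPlay it damages itself by its life minus 100, apparently starting unfinished until BuildSuceess.
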(event `SetTarget`
  (params (Target :type "Actor Object Reference"))
  (`/Engine/EditorBlueprintResources/StandardMacros.IsValid` Target
    (:`Is Valid`
      (set `self.Target` Target)
      (`self.Attack`))))

(event `Attack`
  (bind _returnvalue (`KismetSystemLibrary.K2_SetTimerDelegate` (delegate `Hit`) (`self.TimeRechage`) true))
  (set `self.AttackTimer` _returnvalue)
  (`self.Hit`))

(event `self.ReceiveBeginPlay`
  (`parent.ReceiveBeginPlay`)
  (`KismetSystemLibrary.Delay` 0.2)
  (`GameplayStatics.ApplyDamage` self (- (`/Game/MiniKingdom/Blueprint/Components/BP_Life.Life` (`self.BP_Life`)) 100.0)))

(event `Hit`
  (bind _returnvalue (`SceneComponent.K2_GetComponentLocation` (`self.SpawnArrow`)))
  (bind _target (`self.Target`)
    (:`then`
      (`|SpawnActorFromClass` "/Game/MiniKingdom/Blueprint/Attack/BP_HitArrow.BP_HitArrow_C" (`KismetMathLibrary.MakeTransform` _returnvalue (`KismetMathLibrary.FindLookAtRotation` _returnvalue (`self.K2_GetActorLocation` (`self.Target`)))) "AlwaysSpawn" "MultiplyWithRoot" self (`self.Damage`) _target null))
    (:`else`
      (`KismetSystemLibrary.K2_ClearAndInvalidateTimerHandle` (`self.AttackTimer`))
      (`self.FindTarget`))))

(event `self.Visible.OnComponentBeginOverlap`
  (params (OverlappedComponent :type "PrimitiveComponent Object Reference") (OtherActor :type "Actor Object Reference") (OtherComp :type "PrimitiveComponent Object Reference") (OtherBodyIndex :type Integer) (bFromSweep :type Boolean) (SweepResult :type "HitResult Structure (by ref)"))
  (if (`self.Build`)
    (`self.Target`
      (:`then`)
      (:`else`
        (`self.SetTarget` OtherActor)))))

(event `FindTarget`
  (`self.SetTarget` (`.ReturnValue` (`GameplayStatics.FindNearestActor` (`self.K2_GetActorLocation`) (`PrimitiveComponent.GetOverlappingActors` (`self.Visible`) "/Script/Engine.Actor")))))

(event `self.Visible.OnComponentEndOverlap`
  (params (OverlappedComponent :type "PrimitiveComponent Object Reference") (OtherActor :type "Actor Object Reference") (OtherComp :type "PrimitiveComponent Object Reference") (OtherBodyIndex :type Integer))
  (if (== OtherActor (`self.Target`))
    (set `self.Target` null)
    (`KismetSystemLibrary.K2_ClearAndInvalidateTimerHandle` (`self.AttackTimer`))
    (`self.FindTarget`)))

(event `self.BuildSuceess`
  (`self.FindTarget`))

(fn `UserConstructionScript`
  (`parent.UserConstructionScript`))