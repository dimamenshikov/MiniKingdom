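; Base friendly building that trains warriors for gold from the player's MainCastle in MiniKingdom.
; On its button press, after a short delay, it spawns a warrior at the Entrance if the castle has enough gold and the unit cap is not reached.
; It deducts the cost, plays a sound and updates the name and count label.
; Each warrior's death event frees a slot and refreshes the label.
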(event `self.ButtonPressed_0`
  (`KismetSystemLibrary.Delay` 0.5)
  (bind _maincastle (`/Game/MiniKingdom/Blueprint/DataAsset/PDA_Level.MainCastle` (`/Game/MiniKingdom/Blueprint/DataAsset/PDA_GameplayClasses.Level` (`self.GameplayClasses`)))
    (:`then`
      (if (and (>= (`/Game/MiniKingdom/Blueprint/Environment/BP_BaseFriendBuilding.Gold` _maincastle) (`self.CostWarrior`)) (< (`self.Quantity`) (`self.QuantityBorder`)))
        (bind _returnvalue (`|SpawnActorFromClass` (`self.WarriorClass`) (`SceneComponent.K2_GetComponentToWorld` (`self.Entrance`)) "AlwaysSpawn" "MultiplyWithRoot" null self null))
        (add `/Game/MiniKingdom/Blueprint/Components/BP_Life.OnDeath` (`/Game/MiniKingdom/AI/BP_BaseCharacter.BP_Life` _returnvalue) (delegate `WarriorDeath`))
        (`self.AddGold` (`/Game/MiniKingdom/Blueprint/DataAsset/PDA_Level.MainCastle` (`/Game/MiniKingdom/Blueprint/DataAsset/PDA_GameplayClasses.Level` (`self.GameplayClasses`))) (`self.CostWarrior`) false)
        (`/Engine/EditorBlueprintResources/StandardMacros.IncrementInt` (`self.Quantity`)
          (:`  `
            (`GameplayStatics.PlaySound2D` "/Game/MiniKingdom/Assets/Sound/A_NewWarrior.A_NewWarrior" 1.0 1.0 0.0 null null)
            (set `TextBlock.Text` (`|FormatText` "{Name}          {Quantity}/{QuantityBorder}" (`self.Name`) (`self.Quantity`) (`self.QuantityBorder`)) (`/Game/MiniKingdom/Widgets/WBP_AdvancedInfo.Name` (`self.WidgetObjectDopInfo`)) :!label _label)))))
    (:`else`)))

(event `WarriorDeath`
  (params (Life :type "/Game/MiniKingdom/Blueprint/Components/BP_Life Object Reference"))
  (`/Engine/EditorBlueprintResources/StandardMacros.DecrementInt` (`self.Quantity`)
    (:`  `
      (goto _label))))

(fn `UserConstructionScript`
  (`parent.UserConstructionScript`))