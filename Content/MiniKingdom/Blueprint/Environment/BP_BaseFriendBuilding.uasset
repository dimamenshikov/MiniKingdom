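; Base class for friendly kingdom buildings that start under construction, earn gold once built, and show a selection panel.
; BeginPlay damages the building down to 100 life; damage events later mark it built upon reaching max health, triggering a sound and BuildSuceess hook.
; MainCastle's new-day event adds gold at set intervals; death removes it from the castle's list.
; Clicks toggle its widget in the interface switcher; three empty button events serve as hooks.
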(event `self.ReceiveBeginPlay`
  (`parent.ReceiveBeginPlay`)
  (bind _returnvalue (`|CreateWidget` (`self.WidgetClassInfo`) null self))
  (set `self.WidgetObjectInfo` _returnvalue)
  (bind _maincastle (`/Game/MiniKingdom/Blueprint/DataAsset/PDA_Level.MainCastle` (`/Game/MiniKingdom/Blueprint/DataAsset/PDA_GameplayClasses.Level` (`self.GameplayClasses`)))
    (:`then`
      (set `self.DaySpawn` (`/Game/MiniKingdom/Blueprint/Environment/FriendBuilding/BP_MainCastle.Day` _maincastle))
      (add `/Game/MiniKingdom/Blueprint/Environment/FriendBuilding/BP_MainCastle.OnNewDay` _maincastle (delegate `NewDay`)))
    (:`else`
      _))
  (`KismetSystemLibrary.Delay` 0.0)
  (`GameplayStatics.ApplyDamage` self (- (`/Game/MiniKingdom/Blueprint/Components/BP_Life.Life` (`self.BP_Life`)) 100.0))
  (`KismetSystemLibrary.Delay` 1.0)
  (`ActorComponent.K2_DestroyComponent` (`self.AreaView`)))

(event `NewDay`
  (params (Day :type Integer))
  (if (and (`self.Build`) (== (mod (- Day (`self.DaySpawn`)) (`self.DelayBeetwinIncreaseGold`)) 0))
    (`self.AddGold` (`self.DeltaIncrease`) true)))

(event `/Game/MiniKingdom/Blueprint/Inteface/BPI_Click.LeftClick`
  (params (Interface :type "/Game/MiniKingdom/Widgets/WBP_Interface Object Reference") (Active :type Boolean))
  (bind _widgetswitcher (`/Game/MiniKingdom/Widgets/WBP_Interface.WidgetSwitcher` Interface))
  (bind _widgetobjectinfo (`self.WidgetObjectInfo`))
  (if (`self.Build`)
    (`parent.LeftClick` Interface Active)
    (bind _widgetobjectinfo_2 (`self.WidgetObjectInfo`)
      (:`then`
        (if (and (not (`PanelWidget.HasChild` _widgetswitcher _widgetobjectinfo_2)) Active)
          (`PanelWidget.AddChild` _widgetswitcher _widgetobjectinfo)
          (set `WidgetSwitcher.ActiveWidgetIndex` (`PanelWidget.GetChildIndex` _widgetswitcher _widgetobjectinfo) _widgetswitcher)
          (else
            (`Widget.RemoveFromParent` _widgetobjectinfo)
            (set `WidgetSwitcher.ActiveWidgetIndex` 0 _widgetswitcher))))
      (:`else`))))

(event `ButtonPressed_0`)

(event `ButtonPressed_1`)

(event `ButtonPressed_2`)

(event `self.ReceiveAnyDamage`
  (params (Damage :type "Float (single-precision)") (DamageType :type "DamageType Object Reference") (InstigatedBy :type "Controller Object Reference") (DamageCauser :type "Actor Object Reference"))
  (`parent.ReceiveAnyDamage` Damage DamageType InstigatedBy DamageCauser)
  (if (> Damage 0.0)
    (`self.OnAttack` self))
  (`KismetSystemLibrary.Delay` 0.2)
  (if (`self.Build`)
    _
    (elif (`/Game/MiniKingdom/Blueprint/Components/BP_Life.IsMaxHealth` (`self.BP_Life`))
      (set `self.Build` true)
      (`GameplayStatics.PlaySound2D` "/Game/MiniKingdom/Assets/Sound/A_NewBuilding.A_NewBuilding" 1.0 1.0 0.0 null null)
      (`self.BuildSuceess`))))

(event `BuildSuceess`)

(event `self.Death`
  (bind _maincastle (`/Game/MiniKingdom/Blueprint/DataAsset/PDA_Level.MainCastle` (`/Game/MiniKingdom/Blueprint/DataAsset/PDA_GameplayClasses.Level` (`self.GameplayClasses`)))
    (:`then`
      (`KismetArrayLibrary.Array_RemoveItem` (`/Game/MiniKingdom/Blueprint/Environment/FriendBuilding/BP_MainCastle.Building` _maincastle) self)
      (`parent.Death`))
    (:`else`)))

(fn `AddGold`
  (params (Delta :type Integer) (Add :type Boolean))
  (bind _gold (`self.Gold`))
  (set `self.Gold` (`KismetMathLibrary.SelectInt` (+ Delta _gold) (- _gold Delta) Add)))

(fn `UserConstructionScript`
  (`parent.UserConstructionScript`))