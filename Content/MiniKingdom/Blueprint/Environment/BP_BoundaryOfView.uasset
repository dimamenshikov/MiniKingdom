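; BP_BoundaryOfView is an actor that outlines the player's view footprint on the ground, drawn as four stretched meshes at a fixed high altitude.
; Each tick it finds where the pawn's pitch and yaw meet Z=0, offsets that point by right and up vectors at a 16:9 ratio, then projects the four corners onto the ground.
; DrawBoundaryOfView centers, rotates and scales each construction-spawned mesh along one edge.
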(event `self.ReceiveTick`
  (params (DeltaSeconds :type "Float (single-precision)"))
  (bind _playerlocation (`self.PlayerLocation`))
  (bind (_playerrotation_roll _playerrotation_pitch _playerrotation_yaw) (`KismetMathLibrary.BreakRotator` (`self.PlayerRotation`)))
  (bind _p (`/Game/MiniKingdom/Blueprint/DataAsset/PDA_GameplayClasses.P` (`self.GameplayClasses`)))
  (bind _p_2 (`/Game/MiniKingdom/Blueprint/DataAsset/PDA_GameplayClasses.P` (`self.GameplayClasses`)))
  (bind (_returnvalue_x _returnvalue_y) (`KismetMathLibrary.BreakVector` (+ (`self.PlayerLocation`) (`KismetMathLibrary.GreaterGreater_VectorRotator` (`KismetMathLibrary.MakeVector` (`KismetMathLibrary.Abs` (/ (.z (`self.PlayerLocation`)) (`KismetMathLibrary.DegTan` _playerrotation_pitch)))) (`KismetMathLibrary.MakeRotator` 0.0 0.0 _playerrotation_yaw)))))
  (set `self.PlayerLocation` (`self.K2_GetActorLocation` _p))
  (set `self.PlayerRotation` (`self.K2_GetActorRotation` _p))
  (`KismetArrayLibrary.Array_Clear` (`self.Points`))
  (for _index (range 2)
    (bind _output_get (set `self.Intersection` (`KismetMathLibrary.MakeVector` _returnvalue_x _returnvalue_y)))
    (for _index_2 (range 2)
      (bind _returnvalue (`KismetMathLibrary.VSize` (- _output_get (`self.PlayerLocation`))))
      (bind _returnvalue_2 (- (* _index 2) 1))
      (bind (_returnvalue_x_2 _returnvalue_y_2 _returnvalue_z) (`KismetMathLibrary.BreakVector` (- (+ (+ (`self.Intersection`) (* (`self.GetActorRightVector` _p_2) _returnvalue _returnvalue_2)) (* (`self.GetActorUpVector` _p_2) (/ _returnvalue 1.777778) (- (* _index_2 2) 1) _returnvalue_2)) _playerlocation)))
      (`KismetArrayLibrary.Array_Add` (`self.Points`) (+ _playerlocation (* (`KismetMathLibrary.Abs` (/ (.z _playerlocation) _returnvalue_z)) (`KismetMathLibrary.MakeVector` _returnvalue_x_2 _returnvalue_y_2 _returnvalue_z))))))
  (`self.DrawBoundaryOfView` (`self.Points`)))

(fn `DrawBoundaryOfView`
  (params (FourPoints :type "Array of Vector Structure"))
  (locals (NewLocalVar :type "Float (double-precision)"))
  (for (_array_element _array_index) (`self.Cubes`)
    (bind _output (`|GetArrayItem` FourPoints _array_index))
    (bind _output_2 (`|GetArrayItem` FourPoints (mod (+ _array_index 1) (`KismetArrayLibrary.Array_Length` FourPoints))))
    (bind _returnvalue (/ (+ _output _output_2) 2.0))
    (`SceneComponent.K2_SetWorldTransform` _array_element (`KismetMathLibrary.MakeTransform` (`KismetMathLibrary.MakeVector` (.x _returnvalue) (.y _returnvalue) 8000.0) (`KismetMathLibrary.FindLookAtRotation` _returnvalue _output_2) (`KismetMathLibrary.MakeVector` (/ (`KismetMathLibrary.VSize` (- _output _output_2)) 100.0) 1.0 1.0)) false false)))

(fn `UserConstructionScript`
  (for _ (range 4)
    (bind _returnvalue (`AddComponent|NODE_AddStaticMeshComponent-2` :`bManualAttachment` true :`RelativeTransform` (`KismetMathLibrary.MakeTransform` (- (`self.K2_GetActorLocation`) (0.0 0.0 500.0)) (struct) (1.0 0.25 0.25))))
    (`KismetArrayLibrary.Array_Add` (`self.Cubes`) _returnvalue)))