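; BP_ZoneInvisibility is a level-sized cover volume that is carved away where objects on a custom collision channel overlap it, like fog of war.
; BeginPlay fits one mesh to LevelSize and listens for overlaps.
; Divide works as an on-demand quadtree, replacing each hit block with four half-width children that listen likewise, until blocks at unit scale or below simply vanish.
; Those smallest blocks get a black dynamic material with scale-based opacity.
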(event `self.ReceiveBeginPlay`
  (bind _levelsize (`self.LevelSize`))
  (bind _staticmesh (`self.StaticMesh`))
  (`KismetSystemLibrary.DelayUntilNextTick`)
  (`SceneComponent.K2_SetWorldTransform` _staticmesh (`KismetMathLibrary.MakeTransform` (+ (`self.K2_GetActorLocation`) (`KismetMathLibrary.MakeVector` 0.0 0.0 (/ (.z _levelsize) 2.0))) (`self.K2_GetActorRotation`) (/ _levelsize 100.0)) true false)
  (add `PrimitiveComponent.OnComponentBeginOverlap` _staticmesh (`|CreateDelegate` :!event `Divide`))
  (`PrimitiveComponent.SetCollisionEnabled` _staticmesh "QueryOnly"))

(fn `Divide`
  (params (OverlappedComponent :type "PrimitiveComponent Object Reference") (OtherActor :type "Actor Object Reference") (OtherComp :type "PrimitiveComponent Object Reference") (OtherBodyIndex :type Integer) (bFromSweep :type Boolean) (SweepResult :type "HitResult Structure (by ref)"))
  (locals (Transform :type "Transform Structure"))
  (if (`|EnumEquality` (`PrimitiveComponent.GetCollisionObjectType` OtherComp) "ECC_GameTraceChannel3")
    (bind _output_get (set `local.Transform` (`SceneComponent.K2_GetComponentToWorld` OverlappedComponent)))
    (`ActorComponent.K2_DestroyComponent` OverlappedComponent)
    (bind _x (.x (.scale _output_get)))
    (if (> _x 1.0)
      (for _index (range 4)
        (bind _returnvalue (`AddComponent|NODE_AddStaticMeshComponent-9` :`bManualAttachment` true :`RelativeTransform` (`KismetMathLibrary.MakeTransform` (+ (`KismetMathLibrary.GreaterGreater_VectorRotator` (`KismetMathLibrary.MakeVector` (* _x 25.0 (`KismetMathLibrary.Sqrt` 2.0))) (`KismetMathLibrary.MakeRotator` 0.0 0.0 (- (* (`KismetMathLibrary.Conv_IntToDouble` _index) 90.0) 45.0))) (.location _output_get)) (.rotation _output_get) (`KismetMathLibrary.MakeVector` (/ _x 2.0) (/ (.y (.scale _output_get)) 2.0) (.z (.scale _output_get))))))
        (bind _returnvalue_x (`KismetMathLibrary.BreakVector` (`SceneComponent.K2_GetComponentScale` _returnvalue)))
        (if (not (> _returnvalue_x 1.0))
          (`PrimitiveComponent.SetMaterial` _returnvalue 0 "/Game/MiniKingdom/Assets/GlobalMaterial/MI_Black.MI_Black")
          (bind _returnvalue_2 (`PrimitiveComponent.CreateDynamicMaterialInstance` _returnvalue 0 null "None"))
          (`MaterialInstanceDynamic.SetScalarParameterValue` _returnvalue_2 "Opacity" (* _returnvalue_x 0.5)))
        (add `PrimitiveComponent.OnComponentBeginOverlap` _returnvalue (`|CreateDelegate` :!event `Divide`))
        (`PrimitiveComponent.SetCollisionEnabled` _returnvalue "QueryOnly")))))

(fn `UserConstructionScript`)