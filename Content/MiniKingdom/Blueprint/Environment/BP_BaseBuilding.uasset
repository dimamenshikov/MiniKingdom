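; BP_BaseBuilding is a building base in MiniKingdom with health, a selectable info panel and an explosive death.
; BeginPlay creates the info widget, hands it to BPLife and binds Death, which plays explosion effects and destroys the actor.
; LeftClick adds or removes that widget in the interface's DopInfo slot.
; GetPoint picks a randomized point facing a given position by tracing inward from outside BlockZone, then offsets the hit slightly outward.
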(event `self.ReceiveBeginPlay`
  (bind _bp_life (`self.BP_Life`))
  (bind _returnvalue (`|CreateWidget` (`self.WidgetClassDopInfo`)))
  (bind _output_get (set `self.WidgetObjectDopInfo` _returnvalue))
  (add `/Game/MiniKingdom/Blueprint/Components/BP_Life.OnOwnerDeath` _bp_life (delegate `Death`))
  (set `/Game/MiniKingdom/Blueprint/Components/BP_Life.Widget` _output_get _bp_life)
  (`/Game/MiniKingdom/Widgets/WBP_AdvancedInfo.SetName` _output_get (`self.Name`)))

(event `Death`
  (bind _returnvalue (`self.K2_GetActorLocation`))
  (`GameplayStatics.SpawnEmitterAtLocation` "/Game/MiniKingdom/Assets/Effect/P_Explosion.P_Explosion" _returnvalue (struct) (10.0 10.0 10.0))
  (`GameplayStatics.PlaySoundAtLocation` "/Game/MiniKingdom/Assets/Sound/A_Explosion.A_Explosion" _returnvalue (struct) 1.0 1.0 0.0 null null null null)
  (`self.K2_DestroyActor`))

(event `/Game/MiniKingdom/Blueprint/Inteface/BPI_Click.LeftClick`
  (params (Interface :type "/Game/MiniKingdom/Widgets/WBP_Interface Object Reference") (Active :type Boolean))
  (bind _dopinfo (`/Game/MiniKingdom/Widgets/WBP_Interface.DopInfo` Interface))
  (if (not (`self.bHidden`))
    (bind _widgetobjectdopinfo (`self.WidgetObjectDopInfo`)
      (:`then`
        (if Active
          (`GameplayStatics.PlaySound2D` "/Engine/VREditor/Sounds/UI/Dockable_Window_Pick_Up.Dockable_Window_Pick_Up" 1.0 1.0 0.0 null null)
          (if (not (`PanelWidget.HasChild` (`/Game/MiniKingdom/Widgets/WBP_Interface.DopInfo` Interface) (`self.WidgetObjectDopInfo`)))
            (`PanelWidget.ClearChildren` _dopinfo)
            (`PanelWidget.AddChild` _dopinfo (`self.WidgetObjectDopInfo`)))
          (else
            (`PanelWidget.RemoveChild` _dopinfo _widgetobjectdopinfo))))
      (:`else`))))

(event `self.ReceiveDestroyed`
  (`ActorComponent.K2_DestroyComponent` (`self.BlockZone`)))

(fn `Get Point`
  (params (Point :type "Vector Structure (by ref)"))
  (returns (ReturnValue :type "Vector Structure"))
  (locals (PointTemp :type "Vector Structure"))
  (bind _z (.z Point))
  (bind (_returnvalue_x _returnvalue_y) (`KismetMathLibrary.BreakVector` (`self.K2_GetActorLocation`)))
  (bind (_returnvalue_x_2 _returnvalue_y_2) (`KismetMathLibrary.BreakVector` (`self.K2_GetActorLocation`)))
  (bind (_returnvalue_x_3 _returnvalue_y_3) (`KismetMathLibrary.BreakVector` (`SceneComponent.K2_GetComponentScale` (`self.BlockZone`))))
  (bind _returnvalue (`KismetMathLibrary.MakeVector` (.x (`self.K2_GetActorLocation`)) (.y (`self.K2_GetActorLocation`)) _z))
  (bind _output_get (set `local.PointTemp` (+ (`KismetMathLibrary.GreaterGreater_VectorRotator` (* (+ (* (`KismetMathLibrary.Sqrt` (+ (* _returnvalue_x_3 _returnvalue_x_3) (* _returnvalue_y_3 _returnvalue_y_3))) 50.0) 10.0) (`KismetMathLibrary.Normal` (- Point (`KismetMathLibrary.MakeVector` _returnvalue_x_2 _returnvalue_y_2 _z)))) (`KismetMathLibrary.MakeRotator` 0.0 0.0 (`KismetMathLibrary.RandomFloatInRange` -75.0 75.0))) _returnvalue)))
  (bind _outhit (`KismetSystemLibrary.LineTraceSingle` :`Start` _output_get :`End` _returnvalue :`TraceChannel` "TraceTypeQuery5" :`bIgnoreSelf` false))
  (bind _output_get_2 (set `local.PointTemp` (`.Location` (`GameplayStatics.BreakHitResult` _outhit))))
  (return (+ _output_get_2 (* (`KismetMathLibrary.Normal` (- (`KismetMathLibrary.MakeVector` (.x _output_get_2) (.y _output_get_2)) (`KismetMathLibrary.MakeVector` _returnvalue_x _returnvalue_y))) 20.0))))

(fn `UserConstructionScript`)