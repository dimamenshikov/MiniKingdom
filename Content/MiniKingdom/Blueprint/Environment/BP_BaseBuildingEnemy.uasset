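; Enemy building that starts hidden, is revealed on the first overlap with its Hidden component, and spawns units at its Entrance.
; When AutoSpawn is on, a delayed self-recalling spawn loop fills up to QuantityBorder, and each unit's death schedules another spawn.
; Right-clicking the revealed building creates or removes a BP_BaseTask and shows its widget in the interface.
; On destruction it releases a final QuantityBorder-sized wave of units.
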(event `self.ReceiveBeginPlay`
  (`self.SetActorHiddenInGame` true)
  (`parent.ReceiveBeginPlay`)
  (if (`self.AutoSpawn`)
    (`KismetSystemLibrary.Delay` (`self.Delay`))
    (`self.SpawnActor`)))

(event `Spawn`)

(event `SpawnActor`
  (if (< (`self.Quantity`) (`self.QuantityBorder`))
    (bind _returnvalue (`|SpawnActorFromClass` (`self.Class`) (`SceneComponent.K2_GetComponentToWorld` (`self.Entrance`)) "AlwaysSpawn" "OverrideRootScale" null self null))
    (`/Engine/EditorBlueprintResources/StandardMacros.IncrementInt` (`self.Quantity`)
      (:`  `
        (add `/Game/MiniKingdom/Blueprint/Components/BP_Life.OnDeath` (`/Game/MiniKingdom/AI/BP_BaseCharacter.BP_Life` _returnvalue) (delegate `EnemyDeath`))
        (`KismetSystemLibrary.Delay` (`self.Duration`))
        (`self.SpawnActor`)))))

(event `EnemyDeath`
  (params (Life :type "/Game/MiniKingdom/Blueprint/Components/BP_Life Object Reference"))
  (`/Engine/EditorBlueprintResources/StandardMacros.DecrementInt` (`self.Quantity`)
    (:`  `
      (`KismetSystemLibrary.Delay` (`self.Duration`))
      (`self.SpawnActor`))))

(event `/Game/MiniKingdom/Blueprint/Inteface/BPI_Click.RightClick`
  (params (Interface :type "/Game/MiniKingdom/Widgets/WBP_Interface Object Reference") (Active :type Boolean))
  (bind (_returnvalue_x _returnvalue_y) (`KismetMathLibrary.BreakVector` (`self.K2_GetActorLocation`)))
  (bind _dopinfo (`/Game/MiniKingdom/Widgets/WBP_Interface.DopInfo` Interface))
  (if (not (`self.bHidden`))
    (if Active
      (`self.Task`
        (:`then`
          _)
        (:`else`
          (bind _returnvalue (`|SpawnActorFromClass` "/Game/MiniKingdom/Blueprint/Task/BP_BaseTask.BP_BaseTask_C" (`KismetMathLibrary.MakeTransform` (`KismetMathLibrary.MakeVector` _returnvalue_x _returnvalue_y 90.0)) "AlwaysSpawn" "MultiplyWithRoot" self "NewEnumerator0" null))
          (bind _output_get (set `self.Task` _returnvalue))
          (`SceneComponent.K2_SetRelativeLocation` (`/Game/MiniKingdom/Blueprint/Task/BP_BaseTask.StaticMesh` _output_get) (0.0 0.0 1000.0) false false)))
      (`PanelWidget.ClearChildren` _dopinfo)
      (`PanelWidget.AddChild` _dopinfo (`/Game/MiniKingdom/Blueprint/Task/BP_BaseTask.Widget` _output_get))
      (else
        (bind _task (`self.Task`)
          (:`then`
            (if (`/Game/MiniKingdom/Blueprint/Task/BP_BaseTask.Attach` _task)
              (`PanelWidget.ClearChildren` _dopinfo)
              (else
                (`self.K2_DestroyActor` _task))))
          (:`else`))))))

(event `self.Hidden.OnComponentBeginOverlap`
  (params (OverlappedComponent :type "PrimitiveComponent Object Reference") (OtherActor :type "Actor Object Reference") (OtherComp :type "PrimitiveComponent Object Reference") (OtherBodyIndex :type Integer) (bFromSweep :type Boolean) (SweepResult :type "HitResult Structure (by ref)"))
  (`/Engine/EditorBlueprintResources/StandardMacros.DoOnce` false
    (:`Completed`
      (`self.SetActorHiddenInGame` false))))

(event `self.ReceiveDestroyed`
  (`parent.ReceiveDestroyed`)
  (for _ (range 1 (+ (`self.QuantityBorder`) 1))
    (`|SpawnActorFromClass` (`self.Class`) (`SceneComponent.K2_GetComponentToWorld` (`self.Entrance`)) "AlwaysSpawn" "MultiplyWithRoot" null null null)))

(fn `UserConstructionScript`
  (`parent.UserConstructionScript`))