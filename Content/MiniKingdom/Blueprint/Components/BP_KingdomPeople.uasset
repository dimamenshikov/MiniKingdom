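; Kingdom citizen component that lets a BaseCharacter enter and leave buildings and carry gold between them.
; It registers with the house's main castle on BeginPlay and deregisters when its owner dies.
; GoToHouse walks the character via AI MoveTo to the entrance, hides it, deposits its gold and fires an in-house callback.
; TakeGold empties a building's gold into the carrier, ExitOfHouse restores the character at the entrance, and target-building death is relayed.
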(event `self.ReceiveBeginPlay`
  (bind _asbp_base_character (cast `/Game/MiniKingdom/AI/BP_BaseCharacter` (`self.GetOwner`)))
  (bind _output_get (set `self.BaseCharacter` _asbp_base_character))
  (add `/Game/MiniKingdom/Blueprint/Components/BP_Life.OnOwnerDeath` (`/Game/MiniKingdom/AI/BP_BaseCharacter.BP_Life` _output_get) (delegate `OwnerDeath`))
  (bind _house (`/Game/MiniKingdom/AI/BP_BaseCharacter.House` _output_get)
    (:`then`
      (bind _maincastle (`/Game/MiniKingdom/Blueprint/DataAsset/PDA_Level.MainCastle` (`/Game/MiniKingdom/Blueprint/DataAsset/PDA_GameplayClasses.Level` (`/Game/MiniKingdom/Blueprint/Environment/BP_BaseBuilding.GameplayClasses` _house)))
        (:`then`
          (bind _output_get_2 (set `self.Main Castle` _maincastle))
          (`KismetArrayLibrary.Array_Add` (`/Game/MiniKingdom/Blueprint/Environment/FriendBuilding/BP_MainCastle.KingdomPeople` _output_get_2) self))
        (:`else`)))
    (:`else`)))

(event `OwnerDeath`
  (`KismetArrayLibrary.Array_RemoveItem` (`/Game/MiniKingdom/Blueprint/Environment/FriendBuilding/BP_MainCastle.KingdomPeople` (`self.Main Castle`)) self))

(event `ExitOfHouse`
  (bind _inbuilding (`self.InBuilding`)
    (:`then`
      (bind (_returnvalue_location _returnvalue_rotation) (`KismetMathLibrary.BreakTransform` (`SceneComponent.K2_GetComponentToWorld` (`/Game/MiniKingdom/Blueprint/Environment/BP_BaseBuilding.Entrance` _inbuilding))))
      (`Actor.K2_SetActorLocationAndRotation` (`self.BaseCharacter`) _returnvalue_location _returnvalue_rotation false false)
      (`self.HiddenCharacter` false)
      (set `self.InBuilding` null))
    (:`else`)))

(event `HiddenCharacter`
  (params (Hidden :type Boolean))
  (bind _basecharacter (`self.BaseCharacter`))
  (`Actor.SetActorHiddenInGame` _basecharacter Hidden)
  (`Actor.SetActorEnableCollision` _basecharacter (not Hidden))
  (set `CharacterMovementComponent.GravityScale` (`KismetMathLibrary.Conv_BoolToDouble` Hidden) (`Character.CharacterMovement` _basecharacter)))

(event `GoToHouse`
  (params (House :type "/Game/MiniKingdom/Blueprint/Environment/BP_BaseFriendBuilding Object Reference"))
  (`/Engine/EditorBlueprintResources/StandardMacros.IsValid` House
    (:`Is Valid`
      (if (!= House (`self.InBuilding`))
        (set `self.Target` House)
        (add `/Game/MiniKingdom/Blueprint/Components/BP_Life.OnDeath` (`/Game/MiniKingdom/Blueprint/Environment/BP_BaseBuilding.BP_Life` House) (delegate `TargetBuildingDeath`))
        (set `/Game/MiniKingdom/AI/BP_BaseCharacter.Fight` false (`self.BaseCharacter`))
        (set `CharacterMovementComponent.MaxWalkSpeed` (`self.WalkSpeed`) (`Character.CharacterMovement` (`self.BaseCharacter`)))
        (`self.HiddenCharacter` false)
        (`|AIMoveTo` (`self.BaseCharacter`) (`SceneComponent.K2_GetComponentLocation` (`/Game/MiniKingdom/Blueprint/Environment/BP_BaseBuilding.Entrance` House)) null 10.0
          (:`OnSuccess`
            (bind _target (`self.Target`)
              (:`then`
                (remove `/Game/MiniKingdom/Blueprint/Components/BP_Life.OnDeath` (`/Game/MiniKingdom/Blueprint/Environment/BP_BaseBuilding.BP_Life` _target) (`|CreateDelegate` :!event `TargetBuildingDeath`)))
              (:`else`
                _))
            (`self.HiddenCharacter` true)
            (set `self.InBuilding` _target)
            (`self.GiveGold`)
            (`self.OnInHouse`)))
        (else
          (`self.OnInHouse`))))))

(event `TargetBuildingDeath`
  (params (Life :type "/Game/MiniKingdom/Blueprint/Components/BP_Life Object Reference"))
  (set `self.InBuilding` null)
  (`self.OnBuildingDeath`))

(event `TakeGold`
  (params (Building :type "/Game/MiniKingdom/Blueprint/Environment/BP_BaseFriendBuilding Object Reference"))
  (bind _gold (`/Game/MiniKingdom/Blueprint/Environment/BP_BaseFriendBuilding.Gold` Building))
  (set `self.Gold` (+ _gold (`self.Gold`)))
  (`/Game/MiniKingdom/Blueprint/Environment/BP_BaseFriendBuilding.AddGold` Building _gold false))

(event `GiveGold`
  (bind _gold (`self.Gold`))
  (bind _inbuilding (`self.InBuilding`)
    (:`then`
      (`/Game/MiniKingdom/Blueprint/Environment/BP_BaseFriendBuilding.AddGold` _inbuilding _gold true)
      (`self.RemoveGold` _gold))
    (:`else`)))

(fn `AddGold`
  (params (Gold :type Integer))
  (set `self.Gold` (+ Gold (`self.Gold`))))

(fn `RemoveGold`
  (params (Delta :type Integer))
  (set `self.Gold` (- (`self.Gold`) Delta)))