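; BP_Life is an actor component that tracks its owner's life in MiniKingdom and shows it on health widgets colored or styled by a Friend flag.
; Owner damage lowers the clamped Life, refreshes the widgets and fires update events, plus death events near zero.
; Tick turns the owner's WidgetComponent and its parent toward the player pawn.
; Health() fully heals by applying negative MaxLife damage through the same path.
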(event `self.ReceiveBeginPlay`
  (bind _returnvalue (`self.GetOwner`))
  (bind _friend (`self.Friend`))
  (bind _returnvalue_2 (`Actor.GetComponentByClass` _returnvalue "/Script/UMG.WidgetComponent"))
  (set `self.Life` (`self.MaxLife`))
  (add `Actor.OnTakeAnyDamage` _returnvalue (delegate `OwnerDamaged`))
  (set `self.WidgetComponent` _returnvalue_2)
  (`KismetSystemLibrary.DelayUntilNextTick`)
  (bind _aswbp_health (cast `/Game/MiniKingdom/Widgets/WBP_Health` (`WidgetComponent.GetUserWidgetObject` _returnvalue_2)))
  (bind _output_get (set `self.As WBP Health` _aswbp_health))
  (`KismetSystemLibrary.DelayUntilNextTick`)
  (`/Game/MiniKingdom/Widgets/WBP_Health.SetPercent` _output_get (/ (`self.Life`) (`self.MaxLife`)) _friend)
  (`/Game/MiniKingdom/Widgets/WBP_AdvancedInfo.SetPersent` (`self.Widget`) _friend (`self.Life`) (`self.MaxLife`)))

(event `OwnerDamaged`
  (params (DamagedActor :type "Actor Object Reference") (Damage :type "Float (single-precision)") (DamageType :type "DamageType Object Reference") (InstigatedBy :type "Controller Object Reference") (DamageCauser :type "Actor Object Reference"))
  (bind _life (`self.Life`))
  (bind _life_2 (`self.Life`))
  (bind _friend (`self.Friend`))
  (set `self.LifeTemp` _life)
  (bind _output_get (set `self.Life` (`KismetMathLibrary.FClamp` (- _life Damage) 0.0 (`self.MaxLife`))))
  (`self.OnUpdateLife` (`self.LifeTemp`) _output_get self)
  (bind _as_wbp_health (`self.As WBP Health`)
    (:`then`
      (`/Game/MiniKingdom/Widgets/WBP_Health.SetPercent` _as_wbp_health (/ _output_get (`self.MaxLife`)) _friend))
    (:`else`
      _))
  (bind _widget (`self.Widget`)
    (:`then`
      (`/Game/MiniKingdom/Widgets/WBP_AdvancedInfo.SetPersent` _widget _friend _life_2 (`self.MaxLife`)))
    (:`else`
      _))
  (if (< _life_2 0.001)
    (`self.OnOwnerDeath`)
    (`self.OnDeath` self)))

(event `self.ReceiveTick`
  (params (DeltaSeconds :type "Float (single-precision)"))
  (bind _returnvalue (`GameplayStatics.GetPlayerPawn` 0))
  (bind (_returnvalue_roll _returnvalue_pitch _returnvalue_yaw) (`KismetMathLibrary.BreakRotator` (`Actor.K2_GetActorRotation` _returnvalue)))
  (bind _widgetcomponent (`self.WidgetComponent`)
    (:`then`
      (bind (_returnvalue_roll_2 _returnvalue_pitch_2 _returnvalue_yaw_2) (`KismetMathLibrary.BreakRotator` (`KismetMathLibrary.FindLookAtRotation` (`SceneComponent.K2_GetComponentLocation` (`SceneComponent.GetAttachParent` _widgetcomponent)) (`Actor.K2_GetActorLocation` _returnvalue))))
      (`SceneComponent.K2_SetWorldRotation` (`SceneComponent.GetAttachParent` (`self.WidgetComponent`)) (`KismetMathLibrary.MakeRotator` 0.0 0.0 _returnvalue_yaw_2) false false)
      (`SceneComponent.K2_SetWorldRotation` (`self.WidgetComponent`) (`KismetMathLibrary.MakeRotator` 0.0 _returnvalue_pitch_2 (- _returnvalue_yaw 180.0)) false false))
    (:`else`)))

(fn `Health`
  (`GameplayStatics.ApplyDamage` (`self.GetOwner`) (* (`self.MaxLife`) -1.0)))

(fn `IsLive`
  (returns (Life :type Boolean))
  (return (> (`self.Life`) 0.0)))

(fn `IsMaxHealth`
  (returns (Max :type Boolean))
  (return (== (`self.Life`) (`self.MaxLife`))))