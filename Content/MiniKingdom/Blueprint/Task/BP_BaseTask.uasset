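; Base task actor for Attack or Research jobs that offer a gold reward to friendly fighter characters.
; Attack tasks attach to their owner and listen for its death, while Research tasks use a raised blue mesh.
; A gold-task widget handles selection, Install registers with the main castle, and reward increases spend castle gold.
; Fighter overlap pays the reward and destroys the task, clearing character references; deselecting an uninstalled task also destroys it.
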(event `self.ReceiveBeginPlay`
  (bind _returnvalue (`self.GetOwner`))
  (bind _staticmesh (`self.StaticMesh`))
  (bind _returnvalue_2 (`|CreateWidget` "/Game/MiniKingdom/Widgets/WBP_GoldTask.WBP_GoldTask_C" null self))
  (set `self.Widget` _returnvalue_2)
  (`/Game/MiniKingdom/Core/BP_MiniKingdom_PC.SetActiveActor` (`/Game/MiniKingdom/Blueprint/DataAsset/PDA_GameplayClasses.PC` (`self.GameplayClasses`)) self)
  (switch `/Game/MiniKingdom/Blueprint/Enum/E_Taks` (`self.Task`)
    (:`NewEnumerator0`
      (add `/Game/MiniKingdom/Blueprint/Components/BP_Life.OnDeath` (`self.GetComponentByClass` _returnvalue "/Game/MiniKingdom/Blueprint/Components/BP_Life.BP_Life_C") (`|CreateDelegate` :!event `TargetDeath`))
      (`self.K2_AttachToActor` _returnvalue "None" "KeepWorld" "KeepWorld" "KeepWorld"))
    (:`NewEnumerator1`
      (`PrimitiveComponent.SetMaterial` _staticmesh 0 "/Game/MiniKingdom/Assets/GlobalMaterial/MI_Blue.MI_Blue")
      (`SceneComponent.K2_SetRelativeLocation` _staticmesh (0.0 0.0 500.0) false false)))
  (bind _widget (`self.Widget`)
    (:`then`
      (set `TextBlock.Text` (`KismetMathLibrary.SelectText` "Атаковать!" "Исследовать" (`|EnumEquality` (`self.Task`) "NewEnumerator0")) (`/Game/MiniKingdom/Widgets/WBP_GoldTask.Task` _widget)))
    (:`else`)))

(event `ShowWidget`
  (params (Interface :type "/Game/MiniKingdom/Widgets/WBP_Interface Object Reference"))
  (bind _dopinfo (`/Game/MiniKingdom/Widgets/WBP_Interface.DopInfo` Interface))
  (bind _widget (`self.Widget`)
    (:`then`
      (`PanelWidget.ClearChildren` _dopinfo)
      (`PanelWidget.AddChild` _dopinfo _widget))
    (:`else`)))

(event `/Game/MiniKingdom/Blueprint/Inteface/BPI_Click.RightClick`
  (params (Interface :type "/Game/MiniKingdom/Widgets/WBP_Interface Object Reference") (Active :type Boolean))
  (`self.LeftClick` Interface Active))

(event `/Game/MiniKingdom/Blueprint/Inteface/BPI_Click.LeftClick`
  (params (Interface :type "/Game/MiniKingdom/Widgets/WBP_Interface Object Reference") (Active :type Boolean))
  (if Active
    (`self.ShowWidget` Interface)
    (else
      (bind _widget (`self.Widget`)
        (:`then`
          (`Widget.RemoveFromParent` _widget))
        (:`else`
          _))
      (if (not (`self.Attach`))
        (`self.Destroy`)))))

(event `Install`
  (if (not (`self.Attach`))
    (bind _maincastle (`/Game/MiniKingdom/Blueprint/DataAsset/PDA_Level.MainCastle` (`/Game/MiniKingdom/Blueprint/DataAsset/PDA_GameplayClasses.Level` (`self.GameplayClasses`)))
      (:`then`
        (`/Game/MiniKingdom/Blueprint/Environment/FriendBuilding/BP_MainCastle.NewTasks` _maincastle self))
      (:`else`)))
  (set `self.Attach` true))

(event `IncreaseReward`
  (bind _maincastle (`/Game/MiniKingdom/Blueprint/DataAsset/PDA_Level.MainCastle` (`/Game/MiniKingdom/Blueprint/DataAsset/PDA_GameplayClasses.Level` (`self.GameplayClasses`)))
    (:`then`
      (bind _canbuy (`/Game/MiniKingdom/Blueprint/Environment/FriendBuilding/BP_MainCastle.CanBuySimpleObject` _maincastle 100))
      (if _canbuy
        (`/Game/MiniKingdom/Blueprint/Environment/BP_BaseFriendBuilding.AddGold` _maincastle 100 false)
        (set `self.Reward` (+ (`self.Reward`) 100))))
    (:`else`)))

(event `Destroy`
  (bind _outactors (`GameplayStatics.GetAllActorsOfClass` "/Game/MiniKingdom/AI/BP_BaseFightFriendsCharacter.BP_BaseFightFriendsCharacter_C"))
  (for _array_element _outactors
    (`KismetArrayLibrary.Array_RemoveItem` (`/Game/MiniKingdom/AI/BP_BaseFightFriendsCharacter.Tasks` _array_element) self))
  (for _array_element_2 (`self.ActiveCharacter`)
    (`/Engine/EditorBlueprintResources/StandardMacros.IsValid` _array_element_2
      (:`Is Valid`
        (set `/Game/MiniKingdom/AI/BP_BaseFightFriendsCharacter.ActiveTask` null _array_element_2)
        (`/Game/MiniKingdom/AI/BP_BaseFightCharacter.TargetDeath` _array_element_2 null))))
  (bind _widget (`self.Widget`)
    (:`then`
      (`Widget.RemoveFromParent` _widget))
    (:`else`
      _))
  (`self.K2_DestroyActor`))

(event `self.Box.OnComponentBeginOverlap`
  (params (OverlappedComponent :type "PrimitiveComponent Object Reference") (OtherActor :type "Actor Object Reference") (OtherComp :type "PrimitiveComponent Object Reference") (OtherBodyIndex :type Integer) (bFromSweep :type Boolean) (SweepResult :type "HitResult Structure (by ref)"))
  (bind _asbp_base_fight_friends_character (cast `/Game/MiniKingdom/AI/BP_BaseFightFriendsCharacter` OtherActor))
  (`/Game/MiniKingdom/Blueprint/Components/BP_KingdomPeople.AddGold` (`/Game/MiniKingdom/AI/BP_BaseFightFriendsCharacter.BP_FriendCharacter` _asbp_base_fight_friends_character) (`self.Reward`))
  (`self.Destroy`))

(event `TargetDeath`
  (params (Life :type "/Game/MiniKingdom/Blueprint/Components/BP_Life Object Reference"))
  (bind _maincastle (`/Game/MiniKingdom/Blueprint/DataAsset/PDA_Level.MainCastle` (`/Game/MiniKingdom/Blueprint/DataAsset/PDA_GameplayClasses.Level` (`self.GameplayClasses`)))
    (:`then`
      (`KismetArrayLibrary.Array_RemoveItem` (`/Game/MiniKingdom/Blueprint/Environment/FriendBuilding/BP_MainCastle.Tasks` _maincastle) self))
    (:`else`
      _))
  (`self.Destroy`))

(fn `UserConstructionScript`)