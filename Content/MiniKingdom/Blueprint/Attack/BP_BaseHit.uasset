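; BP_BaseHit is an attack actor in MiniKingdom that delivers damage to a target, either instantly or as a homing projectile.
; On BeginPlay it hits immediately at zero speed, or otherwise turns toward the target and advances each frame through a DelayUntilNextTick loop.
; Within one step of the target, it applies damage credited to its owner, spawns an emitter, plays a sound and destroys itself.
; It also destroys itself if the target becomes invalid.
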(event `self.ReceiveBeginPlay`
  (`self.Attack`))

(event `Hit`
  (bind _target (`self.Target`)
    (:`then`
      (`GameplayStatics.ApplyDamage` _target (`self.Damage`) null (`self.GetOwner`))
      (`GameplayStatics.SpawnEmitterAtLocation` (`self.Emitter Template`) (`self.K2_GetActorLocation`))
      (`GameplayStatics.PlaySoundAtLocation` (`self.Sound`) (`self.K2_GetActorLocation`) (struct) 1.0 1.0 0.0 null null null null))
    (:`else`
      _))
  (`self.K2_DestroyActor`))

(event `Attack`
  (bind _returnvalue (* (`GameplayStatics.GetWorldDeltaSeconds`) (`self.Speed`)))
  (if (== (`self.Speed`) 0.0)
    (`self.Hit`)
    (else
      (`self.Target` :!label _label
        (:`then`
          (`self.K2_SetActorRotation` (`KismetMathLibrary.FindLookAtRotation` (`self.K2_GetActorLocation`) (`self.K2_GetActorLocation` (`self.Target`))))
          (`self.K2_AddActorLocalOffset` (`KismetMathLibrary.MakeVector` _returnvalue))
          (if (== (`self.K2_GetActorLocation`) (`self.K2_GetActorLocation` (`self.Target`)) :`ErrorTolerance` _returnvalue)
            (`self.Hit`)
            (else
              (`KismetSystemLibrary.DelayUntilNextTick`)
              (goto _label))))
        (:`else`
          (`self.K2_DestroyActor`))))))

(fn `UserConstructionScript`)