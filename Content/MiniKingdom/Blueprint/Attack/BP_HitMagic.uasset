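; BP_HitMagic is a magic attack actor that deals area damage on impact.
; Hit runs a sphere overlap-style trace at its location and damages actors whose BP_Life Friend value differs from the owner's.
; A TargetDamage flag guarantees a valid Target is damaged even if the trace missed or filtered it out.
; It also spawns explosion particles and sound, then destroys itself.
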(event `self.Hit`
  (bind _returnvalue (`self.K2_GetActorLocation`))
  (bind _returnvalue_2 (`self.GetOwner`))
  (bind _returnvalue_3 (`self.GetComponentByClass` _returnvalue_2 "/Game/MiniKingdom/Blueprint/Components/BP_Life.BP_Life_C"))
  (bind _outhits (`KismetSystemLibrary.SphereTraceMulti` _returnvalue _returnvalue (`self.Radius`) "TraceTypeQuery3"))
  (for _array_element _outhits
    (bind (_bblockinghit _binitialoverlap _time _distance _location _impactpoint _normal _impactnormal _physmat _hitactor) (`GameplayStatics.BreakHitResult` _array_element))
    (`/Engine/EditorBlueprintResources/StandardMacros.IsValid` _hitactor
      (:`Is Valid`
        (`/Engine/EditorBlueprintResources/StandardMacros.IsValid` _returnvalue_2
          (:`Is Valid`
            (bind _returnvalue_4 (`self.GetComponentByClass` _hitactor "/Game/MiniKingdom/Blueprint/Components/BP_Life.BP_Life_C"))
            (`/Engine/EditorBlueprintResources/StandardMacros.IsValid` _returnvalue_4
              (:`Is Valid`
                (`/Engine/EditorBlueprintResources/StandardMacros.IsValid` _returnvalue_3
                  (:`Is Valid`
                    (if (!= (`/Game/MiniKingdom/Blueprint/Components/BP_Life.Friend` _returnvalue_3) (`/Game/MiniKingdom/Blueprint/Components/BP_Life.Friend` _returnvalue_4))
                      (`GameplayStatics.ApplyDamage` _hitactor (`self.Damage`) null (`self.GetOwner`))
                      (if (== _hitactor (`self.Target`))
                        (set `self.TargetDamage` true))))))))))))
  (`GameplayStatics.SpawnEmitterAtLocation` "/Game/MiniKingdom/Assets/Effect/P_Explosion.P_Explosion" (`self.K2_GetActorLocation`))
  (`GameplayStatics.PlaySoundAtLocation` "/Game/MiniKingdom/Assets/Sound/A_MagicHit.A_MagicHit" (`self.K2_GetActorLocation`) (struct) 1.0 1.0 0.0 null null null null)
  (if (not (`self.TargetDamage`))
    (bind _target (`self.Target`)
      (:`then`
        (`GameplayStatics.ApplyDamage` _target (`self.Damage`) null (`self.GetOwner`)))
      (:`else`
        _)))
  (`self.K2_DestroyActor`))

(fn `UserConstructionScript`
  (`parent.UserConstructionScript`))